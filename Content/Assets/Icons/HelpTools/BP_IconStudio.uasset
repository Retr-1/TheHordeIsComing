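; BP_IconStudio is an icon helper that photographs an item mesh with a 2D scene capture on BeginPlay.
; It centres the mesh, offsets the capture along Y, aims it at the mesh with added pitch, and rescales the mesh per axis from its bounds.
; Orthographic width comes from the largest extent measured before rescaling, plus a margin, then one capture fires after debug prints of scale and name.
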(event `self.ReceiveBeginPlay`
  (bind _capture2d (`self.Capture2D`))
  (bind _itemmesh (`self.ItemMesh`))
  (bind _itemmesh_2 (`self.ItemMesh`))
  (bind (_origin _boxextent _sphereradius) (`KismetSystemLibrary.GetComponentBounds` _itemmesh))
  (bind (_returnvalue_roll _returnvalue_pitch _returnvalue_yaw) (`KismetMathLibrary.BreakRotator` (`KismetMathLibrary.FindLookAtRotation` (`SceneComponent.K2_GetComponentLocation` (`self.Capture2D`)) (`SceneComponent.K2_GetComponentLocation` (`self.ItemMesh`)))))
  (bind _returnvalue (/ 0.1 _sphereradius))
  (set `self.MaxExtent` (`KismetMathLibrary.FMax` (.x _boxextent) (.y _boxextent) (.z _boxextent)))
  (`SceneComponent.K2_SetRelativeLocation` _itemmesh (0.0 0.0 0.0) false false)
  (`SceneComponent.K2_SetRelativeLocation` _capture2d (0.0 100.0 0.0) false false)
  (`SceneComponent.K2_SetWorldRotation` _capture2d (`KismetMathLibrary.MakeRotator` _returnvalue_roll (+ _returnvalue_pitch 10.0) _returnvalue_yaw) false false)
  (`SceneComponent.SetRelativeScale3D` _itemmesh_2 (`KismetMathLibrary.MakeVector` (* (.x _boxextent) _returnvalue) (* (.y _boxextent) _returnvalue) (* (.z _boxextent) _returnvalue)))
  (`KismetSystemLibrary.PrintString` (`KismetStringLibrary.Conv_VectorToString` (`SceneComponent.RelativeScale3D` _itemmesh_2)))
  (`KismetSystemLibrary.PrintString` (`KismetSystemLibrary.GetDisplayName` (`self.ItemMesh`)))
  (set `SceneCaptureComponent2D.OrthoWidth` (* (* (`self.MaxExtent`) 2.0) 1.15) (`self.Capture2D`))
  (`SceneCaptureComponent2D.CaptureScene` (`self.Capture2D`)))

(fn `UserConstructionScript`)