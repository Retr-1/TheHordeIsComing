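; BP_CameraRig is a camera rig actor that rotates itself from yaw and pitch values passed to its functions.
; RotateCamera sets world rotation using frame-time-scaled speeds, clamping pitch between MinPitch and MaxPitch and writing zero roll.
; RigTurn and RigLookUp instead add unclamped local rotation on one axis each, both scaled by YawSpeed.
; The event graph and construction script are empty, so rotation depends on external callers.
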(fn `RigLookUp`
  (params (Value :type "Float (double-precision)"))
  (`self.K2_AddActorLocalRotation` (`KismetMathLibrary.MakeRotator` 0.0 (* (`self.YawSpeed`) Value (`GameplayStatics.GetWorldDeltaSeconds`)))))

(fn `RigTurn`
  (params (Value :type "Float (double-precision)"))
  (`self.K2_AddActorLocalRotation` (`KismetMathLibrary.MakeRotator` 0.0 0.0 (* (`self.YawSpeed`) Value (`GameplayStatics.GetWorldDeltaSeconds`)))))

(fn `RotateCamera`
  (params (Yaw :type "Float (double-precision)") (Pitch :type "Float (double-precision)"))
  (bind (_returnvalue_roll _returnvalue_pitch _returnvalue_yaw) (`KismetMathLibrary.BreakRotator` (`self.K2_GetActorRotation`)))
  (bind _returnvalue (`GameplayStatics.GetWorldDeltaSeconds`))
  (`self.K2_SetActorRotation` (`KismetMathLibrary.MakeRotator` 0.0 (`KismetMathLibrary.FClamp` (+ (* Pitch (`self.PitchSpeed`) _returnvalue) _returnvalue_pitch) (`self.MinPitch`) (`self.MaxPitch`)) (+ (* Yaw (`self.YawSpeed`) _returnvalue) _returnvalue_yaw))))

(fn `UserConstructionScript`)