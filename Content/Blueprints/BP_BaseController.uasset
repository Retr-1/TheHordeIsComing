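; BP_BaseController is a player controller that handles look input, camera swapping and map toggling.
; On BeginPlay it adds the base Enhanced Input mapping context and caches the BP_CameraRig tagged CrystalCamera.
; A FlipFlop blends the view between that rig and the controlled pawn, tracking which is active.
; Look input always turns the pawn and also rotates the rig while it is active; the map action calls MapManager.
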(event `self.ReceiveBeginPlay`
  (bind _returnvalue (subsystem `EnhancedInputLocalPlayerSubsystem`))
  (`/Engine/EditorBlueprintResources/StandardMacros.IsValid` _returnvalue
    (:`Is Valid`
      (`EnhancedInputSubsystemInterface.AddMappingContext` _returnvalue "/Game/Inputs/IMC_BaseMapping.IMC_BaseMapping" 0 (struct))
      (bind _outactors (`GameplayStatics.GetAllActorsWithTag` "CrystalCamera"))
      (bind _asbp_camera_rig (cast `/Game/Blueprints/BP_CameraRig` (`|GetArrayItem` _outactors)))
      (set `self.CrystalCamera` _asbp_camera_rig))))

(event `EnhancedInput|/Game/Inputs/IA_SwapCameras`
  (params (ActionValue :type Boolean) (ElapsedSeconds :type "Float (double-precision)") (TriggeredSeconds :type "Float (double-precision)") (InputAction :type "InputAction Object Reference" :default "/Game/Inputs/IA_SwapCameras.IA_SwapCameras"))
  (:`Triggered`
    (`/Engine/EditorBlueprintResources/StandardMacros.FlipFlop`
      (:`A`
        (`self.SetViewTargetWithBlend` (`self.CrystalCamera`) 1.0)
        (set `self.IsUsingAltCam` true))
      (:`B`
        (`self.SetViewTargetWithBlend` (`self.K2_GetPawn`) 1.0)
        (set `self.IsUsingAltCam` false)))))

(event `EnhancedInput|/Game/Inputs/IA_Look`
  (params (ActionValue :type "Vector2D Structure") (ElapsedSeconds :type "Float (double-precision)") (TriggeredSeconds :type "Float (double-precision)") (InputAction :type "InputAction Object Reference" :default "/Game/Inputs/IA_Look.IA_Look"))
  (bind _returnvalue (`self.K2_GetPawn`))
  (bind (_x _y) (`KismetMathLibrary.BreakVector2D` ActionValue))
  (:`Triggered`
    (`Pawn.AddControllerYawInput` _returnvalue _x)
    (`Pawn.AddControllerPitchInput` _returnvalue _y)
    (if (`self.IsUsingAltCam`)
      (`/Game/Blueprints/BP_CameraRig.RotateCamera` (`self.CrystalCamera`) _x _y))))

(event `EnhancedInput|/Game/Inputs/IA_OpenMap`
  (params (ActionValue :type Boolean) (ElapsedSeconds :type "Float (double-precision)") (TriggeredSeconds :type "Float (double-precision)") (InputAction :type "InputAction Object Reference" :default "/Game/Inputs/IA_OpenMap.IA_OpenMap"))
  (:`Triggered`
    (`MapManagerComponent.ToggleMap` (`self.MapManager`))))

(fn `UserConstructionScript`)