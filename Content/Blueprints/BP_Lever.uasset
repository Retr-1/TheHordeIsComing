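; BP_Lever is an interactable lever that flips between two states when its Interact event fires.
; Each interaction toggles TargetState and plays or reverses the PullAnimation timeline, which lerps the Cylinder's pitch to swing it between the two positions.
; When the timeline finishes, it calls ChangedState with the new state, and debug prints show the state and animation alpha.
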(event `/Game/Blueprints/Interfaces/BPI_Interactable.Interact`
  (bind _output_get (set `self.TargetState` (not (`self.TargetState`))))
  (`KismetSystemLibrary.PrintString` (`KismetStringLibrary.Conv_BoolToString` _output_get))
  (if _output_get
    (bind (_direction _alpha) (`Timeline|PullAnimation` :!label _label)
      (:`Update`
        (`SceneComponent.K2_SetRelativeRotation` (`self.Cylinder`) (`KismetMathLibrary.MakeRotator` 0.0 (`KismetMathLibrary.Lerp` 60.0 -60.0 _alpha)) false false)
        (`KismetSystemLibrary.PrintString` (`KismetStringLibrary.Conv_DoubleToString` _alpha)))
      (:`Finished`
        (`self.ChangedState` (`self.TargetState`))))
    (else
      (goto _label :!via `Reverse`))))

(fn `UserConstructionScript`)