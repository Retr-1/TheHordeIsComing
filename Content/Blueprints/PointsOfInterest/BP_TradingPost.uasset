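; Trading post point of interest that sells two random DT_Items entries at random prices, both rolled on BeginPlay.
; Interact opens UW_TradingPost once while IsOpen is false, passes itself as ParentSign, fills names, icons and prices, and enables cursor input.
; BuyItem1 and BuyItem2 check the character's coins, update the count and add to inventory.
; As written, BuyItem2 deducts nothing and grants Item 1.
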(event `self.ReceiveBeginPlay`
  (set `self.Item2ID` 1)
  (set `self.Item2ID` 2)
  (set `self.Item1Price` (`KismetMathLibrary.RandomIntegerInRange` 30 250))
  (set `self.Item2Price` (`KismetMathLibrary.RandomIntegerInRange` 30 250))
  (bind _outrownames (`DataTableFunctionLibrary.GetDataTableRowNames` "/Game/Blueprints/DataStructs/DT_Items.DT_Items"))
  (set `self.Item1Name` (`KismetStringLibrary.Conv_NameToString` (`KismetArrayLibrary.Array_Random` _outrownames)))
  (bind _outrownames_2 (`DataTableFunctionLibrary.GetDataTableRowNames` "/Game/Blueprints/DataStructs/DT_Items.DT_Items"))
  (set `self.Item2Name` (`KismetStringLibrary.Conv_NameToString` (`KismetArrayLibrary.Array_Random` _outrownames_2))))

(event `/Game/Blueprints/Interfaces/BPI_Interactable.Interact`
  (params (Instigator :type "Actor Object Reference"))
  (bind _returnvalue (`GameplayStatics.GetPlayerController` 0))
  (bind _tradingui (`self.TradingUI`))
  (bind _tradingui_2 (`self.TradingUI`))
  (if (not (`self.IsOpen`))
    (set `self.IsOpen` true)
    (bind _returnvalue_2 (`|CreateWidget` "/Game/UI/TradingPost/UW_TradingPost.UW_TradingPost_C"))
    (set `/Game/UI/TradingPost/UW_TradingPost.ParentSign` self _returnvalue_2)
    (set `self.TradingUI` _returnvalue_2)
    (`UserWidget.AddToViewport` _returnvalue_2 0)
    (`TextBlock.SetText` (`/Game/UI/TradingPost/UW_TradingPost.Item2Price` _returnvalue_2) (`KismetTextLibrary.Conv_IntToText` (`self.Item2Price`)))
    (`TextBlock.SetText` (`/Game/UI/TradingPost/UW_TradingPost.Item1Price` _returnvalue_2) (`KismetTextLibrary.Conv_IntToText` (`self.Item1Price`)))
    (set `PlayerController.bShowMouseCursor` true _returnvalue)
    (`WidgetBlueprintLibrary.SetInputMode_GameAndUIEx` _returnvalue null)
    (bind _returnvalue_3 (`|GetDataTableRow` "/Game/Blueprints/DataStructs/DT_Items.DT_Items" (`KismetStringLibrary.Conv_StringToName` (`self.Item1Name`)))
      (:`then`
        (`Image.SetBrushFromTexture` (`/Game/UI/TradingPost/UW_TradingPost.Item1Image` _tradingui_2) (`.Icon_15_47F7B0D3462E90E827B89C9A21C85BF2` (break `/Game/Blueprints/DataStructs/STR_ItemData` _returnvalue_3)) false)
        (`TextBlock.SetText` (`/Game/UI/TradingPost/UW_TradingPost.Item1Name` _tradingui_2) (`.DisplayName_5_393C9BFB470018DD029FFC9DDA998590` (break `/Game/Blueprints/DataStructs/STR_ItemData` _returnvalue_3)))
        (bind _returnvalue_4 (`|GetDataTableRow` "/Game/Blueprints/DataStructs/DT_Items.DT_Items" (`KismetStringLibrary.Conv_StringToName` (`self.Item2Name`)))
          (:`then`
            (`TextBlock.SetText` (`/Game/UI/TradingPost/UW_TradingPost.Item2Name` _tradingui) (`.DisplayName_5_393C9BFB470018DD029FFC9DDA998590` (break `/Game/Blueprints/DataStructs/STR_ItemData` _returnvalue_4)))
            (`Image.SetBrushFromTexture` (`/Game/UI/TradingPost/UW_TradingPost.Item2Image` _tradingui) (`.Icon_15_47F7B0D3462E90E827B89C9A21C85BF2` (break `/Game/Blueprints/DataStructs/STR_ItemData` _returnvalue_4)) false)))))))

(fn `BuyItem1`
  (bind _item1price (`self.Item1Price`))
  (bind _returnvalue (`GameplayStatics.GetActorOfClass` "/Game/Blueprints/BP_BaseCharacter.BP_BaseCharacter_C"))
  (bind _coincount (`/Game/Blueprints/BP_BaseCharacter.CoinCount` _returnvalue))
  (if (>= (- _coincount _item1price) 0)
    (bind _output_get (set `/Game/Blueprints/BP_BaseCharacter.CoinCount` (- _coincount _item1price) _returnvalue))
    (`/Game/Blueprints/BP_BaseCharacter.CoinUpdate` _returnvalue _output_get)
    (`/Game/Blueprints/Interfaces/BPI_Inventory.AddToInventory` (`/Game/Blueprints/BP_BaseCharacter.BPC_InventoryComponent` _returnvalue) (make `/Game/Blueprints/DataStructs/STR_ItemStack` (`KismetStringLibrary.Conv_StringToName` (`self.Item1Name`)) 1))))

(fn `BuyItem2`
  (bind _returnvalue (`GameplayStatics.GetActorOfClass` "/Game/Blueprints/BP_BaseCharacter.BP_BaseCharacter_C"))
  (bind _coincount (`/Game/Blueprints/BP_BaseCharacter.CoinCount` _returnvalue))
  (if (>= (- _coincount (`self.Item2Price`)) 0)
    (bind _output_get (set `/Game/Blueprints/BP_BaseCharacter.CoinCount` (- _coincount 0) _returnvalue))
    (`/Game/Blueprints/BP_BaseCharacter.CoinUpdate` _returnvalue _output_get)
    (`/Game/Blueprints/Interfaces/BPI_Inventory.AddToInventory` (`/Game/Blueprints/BP_BaseCharacter.BPC_InventoryComponent` _returnvalue) (make `/Game/Blueprints/DataStructs/STR_ItemStack` (`KismetStringLibrary.Conv_StringToName` (`self.Item1Name`)) 1))))

(fn `GetInteractHint`
  (returns (InteractHint :type String))
  (return ""))

(fn `UserConstructionScript`)