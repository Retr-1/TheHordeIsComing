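; BP_Graveyard is a point-of-interest actor that populates a graveyard with vampire enemies and loot chests.
; On BeginPlay it spawns four BP_VampireChild actors and two BT_ChestBottom_Master chests at the world locations of named marker components.
; Only marker locations feed the spawn transforms, so marker rotation and scale are not applied.
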(event `self.ReceiveBeginPlay`
  (`|SpawnActorFromClass` "/Game/Blueprints/Enemies/BaseEnemy/Vampire/BP_VampireChild.BP_VampireChild_C" (`KismetMathLibrary.Conv_VectorToTransform` (`SceneComponent.K2_GetComponentLocation` (`self.spawnVampire1`))) "Undefined" "MultiplyWithRoot" null null)
  (`|SpawnActorFromClass` "/Game/Blueprints/Enemies/BaseEnemy/Vampire/BP_VampireChild.BP_VampireChild_C" (`KismetMathLibrary.Conv_VectorToTransform` (`SceneComponent.K2_GetComponentLocation` (`self.spawnVampire2`))) "Undefined" "MultiplyWithRoot" null null)
  (`|SpawnActorFromClass` "/Game/Blueprints/Enemies/BaseEnemy/Vampire/BP_VampireChild.BP_VampireChild_C" (`KismetMathLibrary.Conv_VectorToTransform` (`SceneComponent.K2_GetComponentLocation` (`self.spawnVampire3`))) "Undefined" "MultiplyWithRoot" null null)
  (`|SpawnActorFromClass` "/Game/Blueprints/Enemies/BaseEnemy/Vampire/BP_VampireChild.BP_VampireChild_C" (`KismetMathLibrary.Conv_VectorToTransform` (`SceneComponent.K2_GetComponentLocation` (`self.spawnVampire4`))) "Undefined" "MultiplyWithRoot" null null)
  (`|SpawnActorFromClass` "/Game/Blueprints/Structures/Chests/BT_ChestBottom_Master.BT_ChestBottom_Master_C" (`KismetMathLibrary.Conv_VectorToTransform` (`SceneComponent.K2_GetComponentLocation` (`self.spawnLootChest1`))) "Undefined" "MultiplyWithRoot" null null)
  (`|SpawnActorFromClass` "/Game/Blueprints/Structures/Chests/BT_ChestBottom_Master.BT_ChestBottom_Master_C" (`KismetMathLibrary.Conv_VectorToTransform` (`SceneComponent.K2_GetComponentLocation` (`self.spawnLootChest`))) "Undefined" "MultiplyWithRoot" null null))

(fn `UserConstructionScript`)