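; Shared loot helper functions that choose which item drops from a list of loot options and how many.
; PickRandomLootFromOptions makes a weighted random pick, using each option's Rarity normalized by the total and accumulated against one random roll, with an empty entry as fallback.
; PickRandomDropAmount looks up the item in DT_Items and rolls within its drop range, capping the maximum at MaxStackSize and returning zero for unknown items.
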(fn `PickRandomDropAmount`
  (params (LootData :type "/Game/Blueprints/DataStructs/STR_LootData Structure"))
  (returns (DropAmount :type Integer))
  (bind _returnvalue (`|GetDataTableRow` "/Game/Blueprints/DataStructs/DT_Items.DT_Items" LootData_ItemID_2_A5BDF8B240622703279E9DA29318D74D)
    (:`then`
      (return (`KismetMathLibrary.RandomIntegerInRange` (break `/Game/Blueprints/DataStructs/STR_IntRange` (`.DropRange_7_AA6FB24F45EB495CE99391B2A39645A8` (break `/Game/Blueprints/DataStructs/STR_LootData` LootData))) (`KismetMathLibrary.Min` (`.Max_4_6F6B276C41242A676433559D682A04AE` (break `/Game/Blueprints/DataStructs/STR_IntRange` (`.DropRange_7_AA6FB24F45EB495CE99391B2A39645A8` (break `/Game/Blueprints/DataStructs/STR_LootData` LootData)))) (`.MaxStackSize_12_FEE5D00340162DCB74A361AE2060BD70` (break `/Game/Blueprints/DataStructs/STR_ItemData` _returnvalue))))))
    (:`RowNotFound`
      (return 0))))

(fn `PickRandomLootFromOptions`
  (params (LootData :type "Array of /Game/Blueprints/DataStructs/STR_LootData Structure"))
  (returns (PickedLoot :type "/Game/Blueprints/DataStructs/STR_LootData Structure"))
  (locals (RaritySum :type "Float (double-precision)") (ProbabilitySum :type "Float (double-precision)") (Randf :type "Float (double-precision)"))
  (set `local.RaritySum` 0.0)
  (set `local.ProbabilitySum` 0.0)
  (for _array_element LootData
    (set `local.RaritySum` (+ (`.Rarity_12_32D0ABB246E36A03CCF081B95AF96D65` (break `/Game/Blueprints/DataStructs/STR_LootData` _array_element)) (`local.RaritySum`))))
  (set `local.Randf` (`KismetMathLibrary.RandomFloat`))
  (for _array_element_2 (`local.LootData`)
    (bind _returnvalue (+ (/ (`.Rarity_12_32D0ABB246E36A03CCF081B95AF96D65` (break `/Game/Blueprints/DataStructs/STR_LootData` _array_element_2)) (`local.RaritySum`)) (`local.ProbabilitySum`)))
    (if (<= (`local.Randf`) _returnvalue)
      (return _array_element_2)
      (else
        (set `local.ProbabilitySum` _returnvalue))))
  (return (make `/Game/Blueprints/DataStructs/STR_LootData` "None" (make `/Game/Blueprints/DataStructs/STR_IntRange` 0))))