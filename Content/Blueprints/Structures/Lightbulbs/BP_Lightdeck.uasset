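; BP_Lightdeck is a row of BP_Lightbulb actors whose combined on/off pattern is stored as an integer bitmask.
; BeginPlay collects the bulbs from child actor components; ConstructDeck can build a deck procedurally but is not called here.
; SetState maps each bit to a bulb, Toggle XORs bits into the state, and AreAllActive compares against the all-ones mask.
; An unconnected Debug routine cycles one lit bulb on a looping timer.
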(event `CustomEvent`
  (bind _returnvalue (* (`self.CurrentState`) 2))
  (if (> _returnvalue (`self.GetMaxState`))
    (`self.SetState` 1)
    (else
      (`self.SetState` _returnvalue))))

(event `self.ReceiveBeginPlay`
  (`self.InitFromViewport`))

(fn `AreAllActive`
  (returns (AreAllActive :type Boolean))
  (return (== (`self.CurrentState`) (`self.GetMaxState`))))

(fn `ConstructDeck`
  (bind _returnvalue (`AddComponent|NODE_AddStaticMeshComponent-0` :`RelativeTransform` (`KismetMathLibrary.MakeTransform` (0.0 0.0 0.0) (struct) (`KismetMathLibrary.MakeVector` (* (`self.NumberOfBulbs`) (`self.BulbWidth`)) 0.2 0.2))))
  (`StaticMeshComponent.SetStaticMesh` _returnvalue "/Engine/BasicShapes/Cube.Cube")
  (for _ (range (`self.NumberOfBulbs`))
    (`|SpawnActorFromClass` "/Game/Blueprints/Structures/Lightbulbs/BP_Lightbulb.BP_Lightbulb_C" (`KismetMathLibrary.MakeTransform` (0.0 0.0 0.0)) "Undefined" "MultiplyWithRoot" null null)))

(fn `GetMaxState`
  (returns (Mask :type Integer))
  (return (- (`KismetMathLibrary.FTrunc` (`KismetMathLibrary.MultiplyMultiply_FloatFloat` 2.0 (`KismetMathLibrary.Conv_IntToDouble` (`KismetArrayLibrary.Array_Length` (`self.Bulbs`))))) 1)))

(fn `InitFromViewport`
  (for _array_element (`SceneComponent.GetChildrenComponents` (`self.DefaultSceneRoot`) false)
    (bind _aschild_actor_component (cast `ChildActorComponent` _array_element))
    (bind _asbp_lightbulb (cast `/Game/Blueprints/Structures/Lightbulbs/BP_Lightbulb` (`ChildActorComponent.ChildActor` _aschild_actor_component)))
    (`KismetArrayLibrary.Array_Add` (`self.Bulbs`) _asbp_lightbulb)))

(fn `SetState`
  (params (Mask :type Integer))
  (locals (MaskVar :type Integer))
  (bind _output_get (set `self.CurrentState` Mask))
  (set `local.MaskVar` _output_get)
  (for _array_element (`self.Bulbs`)
    (if (== (`KismetMathLibrary.And_IntInt` (`local.MaskVar`) 1) 0)
      (`/Game/Blueprints/Structures/Lightbulbs/BP_Lightbulb.TurnOff` _array_element)
      (else
        (`/Game/Blueprints/Structures/Lightbulbs/BP_Lightbulb.TurnOn` _array_element)))
    (set `local.MaskVar` (/ (`local.MaskVar`) 2))))

(fn `Toggle`
  (params (State :type Integer))
  (`self.SetState` (`KismetMathLibrary.Xor_IntInt` State (`self.CurrentState`))))

(fn `UserConstructionScript`)