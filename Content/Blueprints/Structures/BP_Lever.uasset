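; BP_Lever is an interactable lever that shows an "E" pull hint and toggles between two states.
; Each Interact flips TargetState and plays or reverses the PullAnimation timeline, which swings the Cylinder's pitch between its two end angles.
; When the timeline finishes, CurrentState catches up to TargetState and the ChangedState dispatcher fires, so listeners hear only completed changes.
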(event `/Game/Blueprints/Interfaces/BPI_Interactable.Interact`
  (params (Instigator :type "Actor Object Reference"))
  (bind _output_get (set `self.TargetState` (not (`self.TargetState`))))
  (if _output_get
    (bind (_direction _alpha) (`Timeline|PullAnimation` :!label _label)
      (:`Update`
        (`SceneComponent.K2_SetRelativeRotation` (`self.Cylinder`) (`KismetMathLibrary.MakeRotator` 0.0 (`KismetMathLibrary.Lerp` 60.0 -60.0 _alpha)) false false))
      (:`Finished`
        (if (!= (`self.TargetState`) (`self.CurrentState`))
          (set `self.CurrentState` (`self.TargetState`))
          (`self.ChangedState` self))))
    (else
      (goto _label :!via `Reverse`))))

(fn `GetInteractHint`
  (returns (InteractHint :type String))
  (return "Press \"E\" to pull"))

(fn `UserConstructionScript`)