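; Spring platform that flings characters standing on it upward with random horizontal velocity.
; Box overlaps maintain the occupant set, and Tick calls Launch whenever CanLaunch passes, though its occupancy and cooldown check appears unconnected.
; Launch throws every occupant, then plays a slowed timeline that stretches the spring mesh vertically through an exponential, clearing occupants and stamping last-use time on each update.
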(event `self.ReceiveBeginPlay`
  (`TimelineComponent.SetPlayRate` (`self.EjectAnimation`) 0.3))

(event `self.ReceiveTick`
  (params (DeltaSeconds :type "Float (single-precision)"))
  (bind _returnvalue (* (- (`KismetMathLibrary.RandomFloat`) 0.5) 10000.0))
  (if (and (> (`BlueprintSetLibrary.Set_Length` (`self.ActorsStandingOnPlatform`)) 0) (> (- (`KismetSystemLibrary.GetGameTimeInSeconds`) (`self.LastUsed`)) (`self.Cooldown`)))
    (bind _result (`BlueprintSetLibrary.Set_ToArray` (`self.ActorsStandingOnPlatform`)))
    (for _array_element _result
      (`Character.LaunchCharacter` _array_element (`KismetMathLibrary.MakeVector` _returnvalue _returnvalue 3000.0) false false))
    (bind (_direction _value) (`Timeline|EjectAnimation` :!via `PlayFromStart`)
      (:`Update`
        (`SceneComponent.SetWorldScale3D` (`self.SimpleSpring`) (`KismetMathLibrary.MakeVector` 1.0 1.0 (`KismetMathLibrary.Exp` _value)))
        (set `self.LastUsed` (`KismetSystemLibrary.GetGameTimeInSeconds`))
        (`BlueprintSetLibrary.Set_Clear` (`self.ActorsStandingOnPlatform`))))))

(event `self.Box.OnComponentBeginOverlap`
  (params (OverlappedComponent :type "PrimitiveComponent Object Reference") (OtherActor :type "Actor Object Reference") (OtherComp :type "PrimitiveComponent Object Reference") (OtherBodyIndex :type Integer) (bFromSweep :type Boolean) (SweepResult :type "HitResult Structure (by ref)"))
  (bind _ascharacter (cast `Character` OtherActor))
  (`BlueprintSetLibrary.Set_Add` (`self.ActorsStandingOnPlatform`) _ascharacter))

(event `self.Box.OnComponentEndOverlap`
  (params (OverlappedComponent :type "PrimitiveComponent Object Reference") (OtherActor :type "Actor Object Reference") (OtherComp :type "PrimitiveComponent Object Reference") (OtherBodyIndex :type Integer))
  (bind _ascharacter (cast `Character` OtherActor))
  (`BlueprintSetLibrary.Set_Remove` (`self.ActorsStandingOnPlatform`) _ascharacter))

(fn `ActivateSpring`)

(fn `UserConstructionScript`)