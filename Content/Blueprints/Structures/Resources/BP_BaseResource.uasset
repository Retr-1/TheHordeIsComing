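; Base harvestable resource actor that loses health when harvested and yields that amount as items.
; Yield scales a random range by matching tool strength, zero below the requirement, plus a chance bare-handed bonus for low-strength resources.
; Items enter the given inventory interface, or spawn as nearby pickups if it is invalid.
; Surviving hits play a squash scale timeline; depleted resources spawn destruction particles and destroy themselves.
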(event `self.ReceiveBeginPlay`
  (set `self.OriginalScale3D` (`self.GetActorScale3D`)))

(event `/Game/Blueprints/Interfaces/BPI_HarvestableResource.Harvest`
  (params (Inventory :type "/Game/Blueprints/Interfaces/BPI_Inventory Interface") (ToolUsed :type "/Game/Blueprints/DataStructs/STR_Tool Structure"))
  (bind _originalscale3d (`self.OriginalScale3D`))
  (bind _droppeditems (`self.Hit` ToolUsed))
  (`self.ManageItemsFromHit` _droppeditems Inventory)
  (if (<= (`self.Health`) 0)
    (`NiagaraFunctionLibrary.SpawnSystemAtLocation` (`self.DestructionParticles`) (`PrimitiveComponent.GetCenterOfMass` (`self.StaticMesh`) "None"))
    (`self.K2_DestroyActor`)
    (else
      (`TimelineComponent.SetPlayRate` (`self.Squash`) 1.2)
      (bind (_direction _alpha) (`Timeline|Squash` :!via `PlayFromStart`)
        (:`Update`
          (`self.SetActorScale3D` (`KismetMathLibrary.VLerp` (* _originalscale3d 0.8) _originalscale3d _alpha)))))))

(fn `DropItems`
  (params (ItemStack :type "/Game/Blueprints/DataStructs/STR_ItemStack Structure"))
  (locals (SpawnRange :type "Float (double-precision)" :default 50.0))
  (bind _spawnrange (`local.SpawnRange`))
  (bind _returnvalue (* _spawnrange -1.0))
  (`|SpawnActorFromClass` "/Game/Blueprints/Items/BP_WorldItemPickup.BP_WorldItemPickup_C" (`KismetMathLibrary.MakeTransform` (+ (`self.K2_GetActorLocation`) (`KismetMathLibrary.MakeVector` (`KismetMathLibrary.RandomFloatInRange` _returnvalue _spawnrange) (`KismetMathLibrary.RandomFloatInRange` _returnvalue _spawnrange) (`local.SpawnRange`)))) "Undefined" "MultiplyWithRoot" null ItemStack null))

(fn `GetBareHandedDropAmount`
  (params (ToolUsed :type "/Game/Blueprints/DataStructs/STR_Tool Structure"))
  (returns (Amount :type Integer))
  (return (`KismetMathLibrary.Conv_BoolToInt` (and (`|EnumEquality` ToolUsed_Category_2_0F4E7FD44D52BAECFF9C928F69734F67 "NewEnumerator2") (> (`KismetMathLibrary.RandomFloat`) 0.7) (<= (`self.StrengthRequiredToHarvest`) 1)))))

(fn `GetHarvestStrength`
  (params (ToolUsed :type "/Game/Blueprints/DataStructs/STR_Tool Structure"))
  (returns (HarvestStrength :type "Float (double-precision)"))
  (bind _returnvalue (/ (`KismetMathLibrary.Conv_IntToDouble` ToolUsed_Strength_5_118BB1D840E45E159447FDB027040ED1) (`KismetMathLibrary.Conv_IntToDouble` (`self.StrengthRequiredToHarvest`))))
  (return (* (`|EnumEquality` (`self.ToolRequiredToHarvest`) ToolUsed_Category_2_0F4E7FD44D52BAECFF9C928F69734F67) (select `bool` (< _returnvalue 1.0) :`false` _returnvalue))))

(fn `GetUsingToolDropAmount`
  (params (ToolUsed :type "/Game/Blueprints/DataStructs/STR_Tool Structure"))
  (returns (Amount :type Integer))
  (bind (_drophealthrange_min _drophealthrange_max) (break `/Game/Blueprints/DataStructs/STR_FloatRange` (`self.DropHealthRange`)))
  (return (`KismetMathLibrary.Round` (* (`KismetMathLibrary.RandomFloatInRange` _drophealthrange_min _drophealthrange_max) (`self.GetHarvestStrength` (`local.ToolUsed`))))))

(fn `Hit`
  (params (ToolUsed :type "/Game/Blueprints/DataStructs/STR_Tool Structure"))
  (returns (DroppedItems :type "/Game/Blueprints/DataStructs/STR_ItemStack Structure"))
  (locals (DroppedQuantity :type Integer))
  (bind _toolused (`local.ToolUsed`))
  (bind _output_get (set `local.DroppedQuantity` (`KismetMathLibrary.Min` (+ (`self.GetUsingToolDropAmount` _toolused) (`self.GetBareHandedDropAmount` _toolused)) (`self.Health`))))
  (set `self.Health` (- (`self.Health`) _output_get))
  (return (make `/Game/Blueprints/DataStructs/STR_ItemStack` (`self.ResourceName`) (`local.DroppedQuantity`))))

(fn `ManageItemsFromHit`
  (params (ItemStack :type "/Game/Blueprints/DataStructs/STR_ItemStack Structure") (Inventory :type "/Game/Blueprints/Interfaces/BPI_Inventory Interface"))
  (if (> (`.Quantity_5_3B35C6F349B84EFE8FEE39A1BBA6E027` (break `/Game/Blueprints/DataStructs/STR_ItemStack` ItemStack)) 0)
    (if (`KismetSystemLibrary.IsValidInterface` Inventory)
      (`/Game/Blueprints/Interfaces/BPI_Inventory.AddToInventory` Inventory ItemStack)
      (else
        (`self.DropItems` ItemStack)))))

(fn `UserConstructionScript`)