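; BP_BaseTree is a harvestable tree resource that randomizes its look and wood tier when play begins.
; A random variant picks one of four meshes, with per-mesh scale and roll corrections for the pine model.
; A separate random tier sets the leaf and trunk materials by slot name, the strength required to harvest, and the tier-numbered wood resource name.
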(event `self.ReceiveBeginPlay`
  (bind _staticmesh (`self.StaticMesh`))
  (bind _returnvalue (+ (`self.Tier`) 1))
  (`parent.ReceiveBeginPlay`)
  (set `self.Variant` (`KismetMathLibrary.RandomInteger` 4))
  (set `self.Tier` (`KismetMathLibrary.RandomInteger` 3))
  (`StaticMeshComponent.SetStaticMesh` (`self.StaticMesh`) (select `int` (`self.Variant`) :`0` "/Game/Assets/Mesh/Trees/treeVar1.treeVar1" :`1` "/Game/Assets/Mesh/Trees/treeVar2.treeVar2" :`2` "/Game/Assets/Mesh/Trees/treeVar3.treeVar3" :`3` "/Game/Assets/Mesh/Trees/Var4/pine_tree.pine_tree" :!type "StaticMesh Object Reference"))
  (`SceneComponent.SetWorldScale3D` _staticmesh (* (`SceneComponent.K2_GetComponentScale` _staticmesh) (select `int` (`self.Variant`) :`0` 100.0 :`1` 100.0 :`2` 100.0 :`3` 5.0)))
  (`SceneComponent.K2_AddLocalRotation` (`self.StaticMesh`) (`KismetMathLibrary.MakeRotator` (select `int` (`self.Variant`) :`0` 0.0 :`1` 0.0 :`2` 0.0 :`3` -90.0 :!type "Float (single-precision)")) false false)
  (`PrimitiveComponent.SetMaterialByName` (`self.StaticMesh`) "Leaves" (select `int` (`self.Tier`) :`0` "/Game/Assets/Mesh/Drops/TreeVar1/LeavesTier1.LeavesTier1" :`1` "/Game/Assets/Mesh/Drops/TreeVar2/LeavesTier2.LeavesTier2" :`2` "/Game/Assets/Mesh/Drops/TreeVar3/LeavesTier3.LeavesTier3" :!type "MaterialInterface Object Reference"))
  (`PrimitiveComponent.SetMaterialByName` (`self.StaticMesh`) "Trunk" (select `int` (`self.Tier`) :`0` "/Game/Assets/Mesh/Drops/TreeVar1/TrunkTier1.TrunkTier1" :`1` "/Game/Assets/Mesh/Drops/TreeVar2/TrunkTier2.TrunkTier2" :`2` "/Game/Assets/Mesh/Drops/TreeVar3/TrunkTier3.TrunkTier3" :!type "MaterialInterface Object Reference"))
  (set `self.StrengthRequiredToHarvest` _returnvalue)
  (set `self.ResourceName` (`KismetStringLibrary.Conv_StringToName` (`KismetTextLibrary.Conv_TextToString` (`|FormatText` "Wood{Tier}" _returnvalue)))))

(fn `UserConstructionScript`
  (`parent.UserConstructionScript`))