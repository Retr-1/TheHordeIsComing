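; Base harvestable resource actor that yields items when hit with a tool and loses health equal to the amount yielded.
; Yield is a random roll scaled by tool strength, zero for wrong or weak tools, with resource name and tool type from getter functions.
; Items go to the supplied inventory, or spawn as nearby pickups without one.
; Surviving hits play a timeline squash; depletion spawns a Niagara effect and destroys the actor.
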(event `self.ReceiveBeginPlay`
  (set `self.OriginalScale3D` (`self.GetActorScale3D`)))

(event `self.Harvest`
  (params (Inventory :type "/Game/Blueprints/Interfaces/BPI_Inventory Interface") (ToolUsed :type "/Game/Blueprints/DataStructs/STR_Tool Structure"))
  (bind _originalscale3d (`self.OriginalScale3D`))
  (bind _droppeditems (`self.Hit` ToolUsed))
  (`self.ManageItemsFromHit` _droppeditems Inventory)
  (if (<= (`self.Health`) 0)
    (`NiagaraFunctionLibrary.SpawnSystemAtLocation` "/Game/FX/NS_RockDestroyed.NS_RockDestroyed" (`PrimitiveComponent.GetCenterOfMass` (`self.StaticMesh`) "None"))
    (`self.K2_DestroyActor`)
    (else
      (`TimelineComponent.SetPlayRate` (`self.Squash`) 1.2)
      (bind (_direction _alpha) (`Timeline|Squash` :!via `PlayFromStart`)
        (:`Update`
          (`self.SetActorScale3D` (`KismetMathLibrary.VLerp` (* _originalscale3d 0.8) _originalscale3d _alpha)))))))

(fn `CanHarvest`
  (params (Tool :type "/Game/Blueprints/DataStructs/STR_Tool Structure"))
  (returns (CanHarvest :type Boolean))
  (return (and (`|EnumEquality` Tool_Category_2_0F4E7FD44D52BAECFF9C928F69734F67 (`self.GetToolRequiredToHarvest`)) (>= Tool_Strength_5_118BB1D840E45E159447FDB027040ED1 (`self.StrengthRequiredToHarvest`)))))

(fn `DropItems`
  (params (ItemStack :type "/Game/Blueprints/DataStructs/STR_ItemStack Structure"))
  (locals (SpawnRange :type "Float (double-precision)" :default 50.0))
  (bind _spawnrange (`local.SpawnRange`))
  (bind _returnvalue (* _spawnrange -1.0))
  (`|SpawnActorFromClass` "/Game/Blueprints/Items/BP_WorldItemPickup.BP_WorldItemPickup_C" (`KismetMathLibrary.MakeTransform` (+ (`self.K2_GetActorLocation`) (`KismetMathLibrary.MakeVector` (`KismetMathLibrary.RandomFloatInRange` _returnvalue _spawnrange) (`KismetMathLibrary.RandomFloatInRange` _returnvalue _spawnrange) (`local.SpawnRange`)))) "Undefined" "MultiplyWithRoot" null ItemStack null))

(fn `GetHarvestStrength`
  (params (ToolUsed :type "/Game/Blueprints/DataStructs/STR_Tool Structure"))
  (returns (HarvestStrength :type "Float (double-precision)"))
  (bind _returnvalue (/ (`KismetMathLibrary.Conv_IntToDouble` ToolUsed_Strength_5_118BB1D840E45E159447FDB027040ED1) (`KismetMathLibrary.Conv_IntToDouble` (`self.StrengthRequiredToHarvest`))))
  (return (* (`|EnumEquality` (`self.GetToolRequiredToHarvest`) ToolUsed_Category_2_0F4E7FD44D52BAECFF9C928F69734F67) (select `bool` (< _returnvalue 1.0) :`false` _returnvalue))))

(fn `GetHealth`
  (returns (Health :type Integer))
  (return (`self.Health`)))

(fn `GetResourceName`
  (returns (ResourceName :type Name))
  (return "None"))

(fn `GetToolRequiredToHarvest`
  (returns (ToolCategory :type "/Game/Blueprints/DataStructs/E_ToolCategory Enum"))
  (return "NewEnumerator0"))

(fn `Hit`
  (params (ToolUsed :type "/Game/Blueprints/DataStructs/STR_Tool Structure"))
  (returns (DroppedItems :type "/Game/Blueprints/DataStructs/STR_ItemStack Structure"))
  (locals (DroppedQuantity :type Integer))
  (bind (_drophealthrange_min _drophealthrange_max) (break `/Game/Blueprints/DataStructs/STR_FloatRange` (`self.DropHealthRange`)))
  (bind _output_get (set `local.DroppedQuantity` (`KismetMathLibrary.Min` (`KismetMathLibrary.Round` (* (`KismetMathLibrary.RandomFloatInRange` _drophealthrange_min _drophealthrange_max) (`self.GetHarvestStrength` (`local.ToolUsed`)))) (`self.Health`))))
  (set `self.Health` (- (`self.Health`) _output_get))
  (return (make `/Game/Blueprints/DataStructs/STR_ItemStack` (`self.GetResourceName`) (`local.DroppedQuantity`))))

(fn `ManageItemsFromHit`
  (params (ItemStack :type "/Game/Blueprints/DataStructs/STR_ItemStack Structure") (Inventory :type "/Game/Blueprints/Interfaces/BPI_Inventory Interface"))
  (if (> (`.Quantity_5_3B35C6F349B84EFE8FEE39A1BBA6E027` (break `/Game/Blueprints/DataStructs/STR_ItemStack` ItemStack)) 0)
    (if (`KismetSystemLibrary.IsValidInterface` Inventory)
      (`/Game/Blueprints/Interfaces/BPI_Inventory.AddToInventory` Inventory ItemStack)
      (else
        (`self.DropItems` ItemStack)))))

(fn `UserConstructionScript`)