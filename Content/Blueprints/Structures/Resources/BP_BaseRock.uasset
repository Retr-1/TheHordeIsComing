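; BP_BaseRock is a harvestable rock resource that randomly becomes one of three ore tiers when play begins.
; The rolled tier selects the static mesh (plain, silver or gold rock), sets the strength required to harvest, and builds the matching tier-numbered ore resource name.
; Harvesting itself is not implemented in these graphs, and the construction script only calls its parent.
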(event `self.ReceiveBeginPlay`
  (bind _returnvalue (+ (`self.Tier`) 1))
  (`parent.ReceiveBeginPlay`)
  (set `self.Tier` (`KismetMathLibrary.RandomInteger` 3))
  (`StaticMeshComponent.SetStaticMesh` (`self.StaticMesh`) (select `int` (`self.Tier`) :`0` "/Game/Assets/Mesh/OreRocks/Rock.Rock" :`1` "/Game/Assets/Mesh/OreRocks/OreRockSilver.OreRockSilver" :`2` "/Game/Assets/Mesh/OreRocks/OreRockGold.OreRockGold" :!type "StaticMesh Object Reference"))
  (set `self.StrengthRequiredToHarvest` _returnvalue)
  (set `self.ResourceName` (`KismetStringLibrary.Conv_StringToName` (`KismetTextLibrary.Conv_TextToString` (`|FormatText` "Ore{tier}" _returnvalue)))))

(fn `UserConstructionScript`
  (`parent.UserConstructionScript`))