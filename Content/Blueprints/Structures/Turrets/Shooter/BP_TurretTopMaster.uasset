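; Master Blueprint for a shooter turret top that aims at and damages actors tagged "Enemy".
; With no valid target, Tick picks the nearest enemy and checks firing range, then keeps that actor without rechecking range while it stays valid.
; The actor interpolates toward the target while the head shows recoil that eases back.
; On a fire timer, Fire adds kick and flags a hit, which Tick applies as direct damage without projectile or trace.
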(event `self.ReceiveTick`
  (params (DeltaSeconds :type "Float (single-precision)"))
  (bind (_returnvalue_x _returnvalue_y _returnvalue_z) (`KismetMathLibrary.BreakVector` (`SceneComponent.K2_GetComponentLocation` (`self.TurretHead`))))
  (bind _returnvalue (`KismetMathLibrary.RInterpTo` (`self.RecoilOffset`) (struct) (`GameplayStatics.GetWorldDeltaSeconds`) (`self.RecoilReturnSpeed`)))
  (bind _returnvalue_2 (+ (`self.LastFired`) (`GameplayStatics.GetWorldDeltaSeconds`)))
  (if (`KismetSystemLibrary.IsValid` (`self.Closest Actor`))
    (set `self.RecoilOffset` _returnvalue :!label _label)
    (set `self.LastFired` _returnvalue_2)
    (if (>= _returnvalue_2 (`self.FireSpeed`))
      (`self.Fire`))
    (`SceneComponent.K2_SetRelativeRotation` (`self.TurretHead`) _returnvalue false false)
    (`self.K2_SetActorRotation` (`KismetMathLibrary.RInterpTo` (`self.K2_GetActorRotation`) (`KismetMathLibrary.MakeRotator` (* (+ (.pitch (`KismetMathLibrary.FindLookAtRotation` (`KismetMathLibrary.MakeVector` _returnvalue_x _returnvalue_y (+ _returnvalue_z (`self.AimHeightOffset`))) (`self.K2_GetActorLocation` (`self.Closest Actor`)))) 0.0) -1.0) 0.0 (+ (.yaw (`KismetMathLibrary.FindLookAtRotation` (`KismetMathLibrary.MakeVector` _returnvalue_x _returnvalue_y (+ _returnvalue_z (`self.AimHeightOffset`))) (`self.K2_GetActorLocation` (`self.Closest Actor`)))) -90.0)) (`GameplayStatics.GetWorldDeltaSeconds`) (`self.AimSpeed`)))
    (if (`self.ApplyHit`)
      (set `self.ApplyHit` false)
      (`GameplayStatics.ApplyDamage` (`self.Closest Actor`) 10.0))
    (else
      (set `self.ClosestDistance` 99999999.0)
      (bind _outactors (`GameplayStatics.GetAllActorsWithTag` "Enemy"))
      (if (not (`KismetArrayLibrary.Array_IsEmpty` _outactors))
        (for _array_element _outactors
          (bind _returnvalue_3 (`self.GetDistanceTo` _array_element (`ActorComponent.GetOwner` (`self.TurretHead`))))
          (if (< _returnvalue_3 (`self.ClosestDistance`))
            (set `self.Closest Actor` _array_element)
            (set `self.ClosestDistance` _returnvalue_3)))
        (if (<= (`self.ClosestDistance`) (`self.FiringRange`))
          (goto _label))))))

(fn `Fire`
  (set `self.RecoilOffset` (`KismetMathLibrary.ComposeRotators` (`self.RecoilOffset`) (`KismetMathLibrary.MakeRotator` (* (`self.KickYaw`) -1.0))))
  (set `self.LastFired` 0.0)
  (set `self.ApplyHit` true))

(fn `UserConstructionScript`)