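; BP_BuildMaster is a turret structure Blueprint that pairs itself with a separately spawned top actor and can be destroyed by damage.
; On BeginPlay it spawns the TurretTop class at its own location and rotation with a reduced fixed scale.
; Any damage lowers its clamped health, and reaching zero destroys the structure, whose Destroyed event also removes the spawned top.
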(event `self.ReceiveBeginPlay`
  (bind _returnvalue (`self.GetTransform`))
  (bind _returnvalue_2 (`|SpawnActorFromClass` (`self.TurretTop`) (`KismetMathLibrary.MakeTransform` (`KismetMathLibrary.MakeVector` (.x (.location _returnvalue)) (.y (.location _returnvalue)) (.z (.location _returnvalue))) (.rotation _returnvalue) (0.3 0.3 0.3)) "Undefined" "MultiplyWithRoot" null null)))

(event `self.ReceiveDestroyed`
  (`self.K2_DestroyActor` (stale `self.ReceiveBeginPlay` _returnvalue_2)))

(event `self.ReceiveAnyDamage`
  (params (Damage :type "Float (single-precision)") (DamageType :type "DamageType Object Reference") (InstigatedBy :type "Controller Object Reference") (DamageCauser :type "Actor Object Reference"))
  (bind _output_get (set `self.CurrentHealth` (`KismetMathLibrary.FClamp` (- (`self.CurrentHealth`) Damage) 0.0 100.0)))
  (if (== _output_get 0.0)
    (`self.K2_DestroyActor`)))

(fn `UserConstructionScript`)