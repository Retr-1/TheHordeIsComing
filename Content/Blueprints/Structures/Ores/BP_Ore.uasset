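; BP_Ore is a harvestable ore node that takes random damage and yields a random quantity of its resource each time it is interacted with.
; Items go straight into the instigator's inventory through BPI_Inventory, or spawn as BP_WorldItemPickup actors scattered nearby if it lacks that interface.
; It destroys itself when health runs out, otherwise plays a timeline-driven squash scale as hit feedback.
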(event `/Game/Blueprints/Interfaces/BPI_Interactable.Interact`
  (params (Instigator :type "Actor Object Reference"))
  (bind _droppeditems (`self.Hit`))
  (`self.ManageItemsFromHit` _droppeditems Instigator)
  (if (<= (`self.Health`) 0.0)
    (`self.K2_DestroyActor`)
    (else
      (bind (_direction _alpha) (`Timeline|Squash` :!via `PlayFromStart`)
        (:`Update`
          (`self.SetActorScale3D` (`KismetMathLibrary.VLerp` (1.0 1.0 1.0) (0.8 0.8 0.8) _alpha)))))))

(fn `DropItems`
  (params (ItemStack :type "/Game/Blueprints/DataStructs/STR_ItemStack Structure"))
  (locals (SpawnRange :type "Float (double-precision)" :default 50.0))
  (bind _spawnrange (`local.SpawnRange`))
  (bind _returnvalue (* _spawnrange -1.0))
  (`|SpawnActorFromClass` "/Game/Blueprints/Items/BP_WorldItemPickup.BP_WorldItemPickup_C" (`KismetMathLibrary.MakeTransform` (+ (`self.K2_GetActorLocation`) (`KismetMathLibrary.MakeVector` (`KismetMathLibrary.RandomFloatInRange` _returnvalue _spawnrange) (`KismetMathLibrary.RandomFloatInRange` _returnvalue _spawnrange) (`local.SpawnRange`)))) "Undefined" "MultiplyWithRoot" null ItemStack null))

(fn `Hit`
  (returns (DroppedItems :type "/Game/Blueprints/DataStructs/STR_ItemStack Structure"))
  (bind (_drophealthrange_min _drophealthrange_max) (break `/Game/Blueprints/DataStructs/STR_FloatRange` (`self.DropHealthRange`)))
  (bind (_dropresourcerange_min _dropresourcerange_max) (break `/Game/Blueprints/DataStructs/STR_IntRange` (`self.DropResourceRange`)))
  (set `self.Health` (- (`self.Health`) (`KismetMathLibrary.RandomFloatInRange` _drophealthrange_min _drophealthrange_max)))
  (return (make `/Game/Blueprints/DataStructs/STR_ItemStack` (`self.OreName`) (`KismetMathLibrary.RandomIntegerInRange` _dropresourcerange_min _dropresourcerange_max))))

(fn `ManageItemsFromHit`
  (params (ItemStack :type "/Game/Blueprints/DataStructs/STR_ItemStack Structure") (Instigator :type "Actor Object Reference"))
  (bind _asbpi_inventory (cast `/Game/Blueprints/Interfaces/BPI_Inventory` Instigator)
    (:`then`
      (`/Game/Blueprints/Interfaces/BPI_Inventory.AddToInventory` _asbpi_inventory ItemStack))
    (:`CastFailed`
      (`self.DropItems` ItemStack))))

(fn `UserConstructionScript`)