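; Master turret top actor that automatically tracks the first "Player"-tagged actor and fires on a timer.
; Each Tick interpolates actor rotation toward that target's bounds center, remapping look-at pitch onto roll with a yaw offset.
; Fire only resets the timer and adds a recoil kick, spawning no projectile or damage.
; Recoil eases back to zero on TurretHead's relative rotation, separate from the aim.
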(event `self.ReceiveTick`
  (params (DeltaSeconds :type "Float (single-precision)"))
  (bind (_returnvalue_x _returnvalue_y _returnvalue_z) (`KismetMathLibrary.BreakVector` (`SceneComponent.K2_GetComponentLocation` (`self.TurretHead`))))
  (bind _returnvalue (`KismetMathLibrary.RInterpTo` (`self.RecoilOffset`) (struct) (`GameplayStatics.GetWorldDeltaSeconds`) (`self.RecoilReturnSpeed`)))
  (bind _returnvalue_2 (+ (`self.LastFired`) (`GameplayStatics.GetWorldDeltaSeconds`)))
  (bind _outactors (`GameplayStatics.GetAllActorsWithTag` "Player"))
  (set `self.RecoilOffset` _returnvalue)
  (set `self.LastFired` _returnvalue_2)
  (if (>= _returnvalue_2 (`self.FireSpeed`))
    (`self.Fire`)
    (`KismetSystemLibrary.PrintString` "FIred"))
  (`SceneComponent.K2_SetRelativeRotation` (`self.TurretHead`) _returnvalue false false)
  (bind _origin (`self.GetActorBounds` (`|GetArrayItem` _outactors) false false))
  (`self.K2_SetActorRotation` (`KismetMathLibrary.RInterpTo` (`self.K2_GetActorRotation`) (`KismetMathLibrary.MakeRotator` (* (+ (.pitch (`KismetMathLibrary.FindLookAtRotation` (`KismetMathLibrary.MakeVector` _returnvalue_x _returnvalue_y (+ _returnvalue_z 220.0)) (`KismetMathLibrary.MakeVector` (.x _origin) (.y _origin) (.z _origin)))) 0.0) -1.0) 0.0 (+ (.yaw (`KismetMathLibrary.FindLookAtRotation` (`KismetMathLibrary.MakeVector` _returnvalue_x _returnvalue_y (+ _returnvalue_z 220.0)) (`KismetMathLibrary.MakeVector` (.x _origin) (.y _origin) (.z _origin)))) -90.0)) (`GameplayStatics.GetWorldDeltaSeconds`) (`self.AimSpeed`))))

(fn `Fire`
  (set `self.RecoilOffset` (`KismetMathLibrary.ComposeRotators` (`self.RecoilOffset`) (`KismetMathLibrary.MakeRotator` (* (`self.KickYaw`) -1.0))))
  (set `self.LastFired` 0.0))

(fn `UserConstructionScript`)