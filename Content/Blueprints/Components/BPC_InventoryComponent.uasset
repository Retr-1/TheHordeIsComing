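; Inventory component that holds a fixed number of item stack slots, padded with empty entries on BeginPlay, and tracks an active hotbar index.
; Adding a stack first tops up matching slots to the data table's max stack size, then puts the remainder in the first empty slot or drops it.
; Slots can be read, set, swapped or emptied, with drops spawning a world pickup actor in front of the owner.
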(event `self.ReceiveBeginPlay`
  (for _ (range (`KismetArrayLibrary.Array_Length` (`self.Items`)) (`self.MaxSlots`))
    (`KismetArrayLibrary.Array_Add` (`self.Items`) (make `/Game/Blueprints/DataStructs/STR_ItemStack` "None"))))

(fn `AddItemStack`
  (params (InputItemStack :type "/Game/Blueprints/DataStructs/STR_ItemStack Structure"))
  (locals (ToRelocate :type Integer) (InputItemQuantityVar :type Integer))
  (bind _resultingitemstack (`self.Fill Partial Slots with Item Stack` InputItemStack))
  (bind _success (`self.AddItemStackToEmptyPlace` _resultingitemstack))
  (if (not _success)
    (`self.DropItemStackFromInput` _resultingitemstack)))

(fn `AddItemStackToEmptyPlace`
  (params (InputItemStack :type "/Game/Blueprints/DataStructs/STR_ItemStack Structure"))
  (returns (Success :type Boolean))
  (locals (IsPlaced :type Boolean))
  (if (not (`/Game/Blueprints/FunctionLibraries/ItemStackHelpers.IsEmpty` InputItemStack))
    (for (_ _array_index) (`self.Items`)
      (if (`self.IsEmptySlot` _array_index)
        (`KismetArrayLibrary.Array_Set` (`self.Items`) _array_index (`local.InputItemStack`))
        (set `local.IsPlaced` true)
        (break)))
    (return (`local.IsPlaced`))))

(fn `DropItemStackFromIndex`
  (params (InputIndex :type Integer))
  (if (`self.IsEmptySlot` InputIndex)
    (`KismetSystemLibrary.PrintString` "NOEPEEE")
    (else
      (bind _itemstack (`self.TakeItemStack` InputIndex))
      (`self.DropItemStackFromInput` _itemstack))))

(fn `DropItemStackFromInput`
  (params (InputItemStack :type "/Game/Blueprints/DataStructs/STR_ItemStack Structure"))
  (bind _returnvalue (`self.GetOwner`))
  (if (not (`/Game/Blueprints/FunctionLibraries/ItemStackHelpers.IsEmpty` InputItemStack))
    (`|SpawnActorFromClass` "/Game/Blueprints/Items/BP_WorldItemPickup.BP_WorldItemPickup_C" (`KismetMathLibrary.MakeTransform` (+ (`Actor.K2_GetActorLocation` _returnvalue) (* (`Actor.GetActorForwardVector` _returnvalue) 300.0))) "Undefined" "MultiplyWithRoot" null InputItemStack null)))

(fn `Fill Partial Slots with Item Stack`
  (params (InputItemStack :type "/Game/Blueprints/DataStructs/STR_ItemStack Structure"))
  (returns (ResultingItemStack :type "/Game/Blueprints/DataStructs/STR_ItemStack Structure"))
  (locals (Quantity :type Integer))
  (bind _inputitemstack_itemid (break `/Game/Blueprints/DataStructs/STR_ItemStack` (`local.InputItemStack`)))
  (set `local.Quantity` InputItemStack_Quantity_5_3B35C6F349B84EFE8FEE39A1BBA6E027)
  (for (_array_element _array_index) (`self.Items`)
    (bind _maxstacksize (`self.GetMaxStackSizeByItemID` (break `/Game/Blueprints/DataStructs/STR_ItemStack` _array_element))
      (:`OutExec`
        (if (== (break `/Game/Blueprints/DataStructs/STR_ItemStack` _array_element) _inputitemstack_itemid)
          (bind (_tomove _newdestinationcount _newsourcecount) (`self.CalculateTransferCounts` (`local.Quantity`) (`.Quantity_5_3B35C6F349B84EFE8FEE39A1BBA6E027` (break `/Game/Blueprints/DataStructs/STR_ItemStack` _array_element)) _maxstacksize))
          (`KismetArrayLibrary.Array_Set` (`self.Items`) _array_index (make `/Game/Blueprints/DataStructs/STR_ItemStack` (break `/Game/Blueprints/DataStructs/STR_ItemStack` _array_element) _newdestinationcount))
          (set `local.Quantity` _newsourcecount)))))
  (return (make `/Game/Blueprints/DataStructs/STR_ItemStack` InputItemStack_ItemID_2_00E5EA564AF4549C4134F1B96064D5C4 (`local.Quantity`))))

(fn `GetItemAtIndex`
  (params (SlotIndex :type Integer))
  (returns (ItemStack :type "/Game/Blueprints/DataStructs/STR_ItemStack Structure"))
  (if (`self.IsSlotIndexValid` SlotIndex)
    (return (`|GetArrayItem` (`self.Items`) SlotIndex))))

(fn `IsEmptySlot`
  (params (Index :type Integer))
  (returns (IsEmpty :type Boolean))
  (bind (_itemstack_itemid _itemstack_quantity) (break `/Game/Blueprints/DataStructs/STR_ItemStack` (`self.GetItemAtIndex` Index)))
  (return (or (== _itemstack_itemid "None") (<= _itemstack_quantity 0))))

(fn `IsSlotIndexValid`
  (params (SlotIndex :type Integer))
  (returns (IsValid :type Boolean))
  (return (and (>= SlotIndex 0) (< SlotIndex (`self.MaxSlots`)))))

(fn `MoveOrSwapItems`
  (params (FromIndex :type Integer) (ToIndex :type Integer))
  (`KismetArrayLibrary.Array_Swap` (`self.Items`) FromIndex ToIndex))

(fn `SetActiveHotbarIndex`
  (params (HotbarIndex :type Integer))
  (set `self.ActiveHotbarIndex` HotbarIndex))

(fn `SetItemAtIndex`
  (params (SlotIndex :type Integer) (Item :type "/Game/Blueprints/DataStructs/STR_ItemStack Structure"))
  (if (`self.IsSlotIndexValid` SlotIndex)
    (`KismetArrayLibrary.Array_Set` (`self.Items`) (`local.SlotIndex`) (`local.Item`))))

(fn `TakeItemStack`
  (params (Index :type Integer))
  (returns (ItemStack :type "/Game/Blueprints/DataStructs/STR_ItemStack Structure"))
  (locals (TmpItem :type "/Game/Blueprints/DataStructs/STR_ItemStack Structure"))
  (bind _output_get (set `local.TmpItem` (`|GetArrayItem` (`self.Items`) Index)))
  (`KismetArrayLibrary.Array_Set` (`self.Items`) Index (make `/Game/Blueprints/DataStructs/STR_ItemStack` "None"))
  (return _output_get))