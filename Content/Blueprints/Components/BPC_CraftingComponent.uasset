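; Actor component that adds recipe crafting to its owner, working on the owner's BPC_InventoryComponent.
; CanCraft compares inventory counts against each recipe requirement; Craft then removes those stacks and adds the product.
; On BeginPlay it creates a hidden WBP_Crafting widget linked to itself.
; Toggling that UI also switches the owning player controller's input mode and mouse cursor.
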(event `self.ReceiveBeginPlay`
  (set `self.Inventory` (`Actor.GetComponentByClass` (`self.GetOwner`) "/Game/Blueprints/Components/BPC_InventoryComponent.BPC_InventoryComponent_C"))
  (bind _returnvalue (`|CreateWidget` "/Game/Blueprints/UserInterface/Crafting/WBP_Crafting.WBP_Crafting_C" null self))
  (bind _output_get (set `self.Widget` _returnvalue))
  (`UserWidget.AddToViewport` _output_get 0)
  (`Widget.SetVisibility` (`self.Widget`) "Hidden"))

(fn `CanCraft`
  (params (Recipe :type "/Game/Blueprints/DataStructs/STR_Recipe Structure"))
  (returns (CanCraft :type Boolean))
  (locals (Can :type Boolean))
  (set `local.Can` true)
  (for _array_element Recipe_Requirements_6_EB08D3554E19F14EFA2EB5BB7B654CB9
    (if (< (`self.GetItemCount` (break `/Game/Blueprints/DataStructs/STR_ItemStack` _array_element)) (`.Quantity_5_3B35C6F349B84EFE8FEE39A1BBA6E027` (break `/Game/Blueprints/DataStructs/STR_ItemStack` _array_element)))
      (set `local.Can` false)))
  (return (`local.Can`)))

(fn `Craft`
  (params (Recipe :type "/Game/Blueprints/DataStructs/STR_Recipe Structure"))
  (bind (_recipe_product _recipe_requirements) (break `/Game/Blueprints/DataStructs/STR_Recipe` (`local.Recipe`)))
  (if (`self.CanCraft` Recipe)
    (for _array_element _recipe_requirements
      (`/Game/Blueprints/Components/BPC_InventoryComponent.RemoveItemStack` (`self.Inventory`) _array_element))
    (`/Game/Blueprints/Components/BPC_InventoryComponent.AddItemStack` (`self.Inventory`) _recipe_product)))

(fn `GetItemCount`
  (params (ItemID :type Name))
  (returns (Count :type Integer))
  (bind _count (`/Game/Blueprints/Interfaces/BPI_Inventory.GetItemCount` (`self.Inventory`) ItemID))
  (return _count))

(fn `SetCraftingUIVisibility`
  (params (Visible :type Boolean))
  (bind _aspawn (cast `Pawn` (`self.GetOwner`)))
  (bind _asplayer_controller (cast `PlayerController` (`Pawn.GetController` _aspawn)))
  (if (`local.Visible`)
    (`WidgetBlueprintLibrary.SetInputMode_GameAndUIEx` _asplayer_controller null)
    (set `PlayerController.bShowMouseCursor` true _asplayer_controller)
    (`Widget.SetVisibility` (`self.Widget`) "Visible")
    (else
      (`WidgetBlueprintLibrary.SetInputMode_GameOnly` _asplayer_controller)
      (set `PlayerController.bShowMouseCursor` false _asplayer_controller)
      (`Widget.SetVisibility` (`self.Widget`) "Hidden"))))

(fn `ToggleCraftingUIVisibility`
  (bind _output_get (set `self.IsUIVisible` (not (`self.IsUIVisible`))))
  (`self.SetCraftingUIVisibility` _output_get))