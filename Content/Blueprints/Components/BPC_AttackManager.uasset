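; BPC_AttackManager is a component that starts montage-based attacks on its owning Character, limited by a cooldown.
; InitializeAttack plays the supplied montage when CanAttack finds that enough game time has passed since the last attack, then records the new attack time.
; The hit functions HitOnce, HitContinuos and DetectHits are empty stubs, and the WeaponMesh input is not yet used.
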(fn `CanAttack`
  (returns (CanAttack :type Boolean))
  (return (> (- (`KismetSystemLibrary.GetGameTimeInSeconds`) (`self.LastAttackedTime`)) (`self.Cooldown`))))

(fn `DetectHits`)

(fn `HitContinuos`)

(fn `HitOnce`)

(fn `InitializeAttack`
  (params (MontageToPlay :type "AnimMontage Object Reference") (WeaponMesh :type "StaticMesh Object Reference"))
  (if (`self.CanAttack`)
    (bind _ascharacter (cast `Character` (`self.GetOwner`)))
    (`Character.PlayAnimMontage` _ascharacter (`local.MontageToPlay`) 1.0 "None")
    (set `self.LastAttackedTime` (`KismetSystemLibrary.GetGameTimeInSeconds`))))