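; BP_BaseMode is a game mode that runs an exploration countdown followed by an enemy wave, and can respawn the player.
; After gathering EnemySpawner actors at start, it resets the exploration timer widget and waits before starting the wave.
; Each wave increments WaveNumber, sets the enemy count to its square, and queues each BP_Enemy on a random spawner.
; RespawnPlayer spawns a new BP_BaseCharacter and possesses it; nothing here restarts the exploration phase.
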(event `self.ReceiveTick`
  (params (DeltaSeconds :type "Float (single-precision)")))

(event `self.ReceiveBeginPlay`
  (`KismetSystemLibrary.Delay` 0.2)
  (bind _outactors (`GameplayStatics.GetAllActorsOfClass` "/Game/Blueprints/Enemies/BaseEnemy/EnemySpawner.EnemySpawner_C"))
  (set `self.Spawners` _outactors)
  (`self.ExploringPhaseStart`))

(event `ExploringPhaseStart`
  (bind _timeperwave (`self.TimePerWave`))
  (bind _foundwidgets (`WidgetBlueprintLibrary.GetAllWidgetsOfClass` "/Game/Blueprints/UserInterface/WB_ExplorationTimer.WB_ExplorationTimer_C"))
  (if (> (`KismetArrayLibrary.Array_Length` _foundwidgets) 0)
    (`/Game/Blueprints/UserInterface/WB_ExplorationTimer.ResetTimer` (`|GetArrayItem` _foundwidgets) _timeperwave))
  (`KismetSystemLibrary.Delay` _timeperwave)
  (`self.WavePhaseStart`))

(event `WavePhaseStart`
  (bind _wavenumber (`self.WaveNumber`))
  (`KismetSystemLibrary.PrintString` (`KismetStringLibrary.Conv_IntToString` _wavenumber))
  (set `self.WaveNumber` (+ _wavenumber 1))
  (`self.GenerateNumberOfEnemies`)
  (`self.SpawnEnemy`))

(event `SpawnEnemy`
  (for _ (range (`self.MaxEnemies`))
    (`/Game/Blueprints/Enemies/BaseEnemy/EnemySpawner.AddEnemyToQueue` (`KismetArrayLibrary.Array_Random` (`self.Spawners`)) "/Game/Blueprints/Enemies/BaseEnemy/BP_Enemy.BP_Enemy_C")))

(event `Respawn Player`
  (params (SpawnTransform :type "Transform Structure"))
  (bind _returnvalue (`|SpawnActorFromClass` "/Game/Blueprints/BP_BaseCharacter.BP_BaseCharacter_C" SpawnTransform "Undefined" "MultiplyWithRoot" null null))
  (`Controller.Possess` (`GameplayStatics.GetPlayerController` 0) _returnvalue))

(fn `GenerateNumberOfEnemies`
  (bind _output_get (set `self.NumberOfEnemies` (`KismetMathLibrary.FTrunc` (`KismetMathLibrary.Square` (`KismetMathLibrary.Conv_IntToDouble` (`self.WaveNumber`))))))
  (set `self.MaxEnemies` _output_get))

(fn `UserConstructionScript`)