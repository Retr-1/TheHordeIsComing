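; Player controller for the character editor screen, which lets the player leave for the PerlinNoise level on confirm.
; On BeginPlay it shows the editor widget in UI-only input, finds the preview actor and switches view to the first CameraActor.
; It seeds the arm and leg sliders from GameInstance proportions, with the leg slider reading LowerRightArmLength.
; Confirming restores game-only input and opens that level without saving anything itself.
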(event `self.ReceiveBeginPlay`
  (bind _widget (`self.Widget`))
  (bind _returnvalue (`|CreateWidget` "/Game/Blueprints/UserInterface/WBP_CharacterEditor.WBP_CharacterEditor_C"))
  (bind _output_get (set `self.Widget` _returnvalue))
  (add `/Game/Blueprints/UserInterface/WBP_CharacterEditor.ConfirmChanges` _output_get (delegate `LeaveEditor`))
  (`UserWidget.AddToViewport` _output_get 0)
  (set `self.bShowMouseCursor` true)
  (`WidgetBlueprintLibrary.SetInputMode_UIOnlyEx` self null)
  (bind _outactors (`GameplayStatics.GetAllActorsOfClass` "/Game/Blueprints/BP_BaseCharacterPreview.BP_BaseCharacterPreview_C"))
  (set `self.PreviewActor` (`|GetArrayItem` _outactors))
  (bind _outactors_2 (`GameplayStatics.GetAllActorsOfClass` "/Script/Engine.CameraActor"))
  (bind _output_get_2 (set `self.CameraActor` (`|GetArrayItem` _outactors_2)))
  (`self.SetViewTargetWithBlend` _output_get_2)
  (bind _asbp_game_instance (cast `/Game/Blueprints/BP_GameInstance` (`GameplayStatics.GetGameInstance`)))
  (bind (_proportions_upperrightarmlength _proportions_lowerrightarmlength) (break `/Game/Blueprints/DataStructs/STR_CharacterProportions` (`/Game/Blueprints/BP_GameInstance.Proportions` _asbp_game_instance)))
  (`Slider.SetValue` (`/Game/Blueprints/UserInterface/WBP_CharacterEditor.SliderArm` _widget) _proportions_upperrightarmlength)
  (`Slider.SetValue` (`/Game/Blueprints/UserInterface/WBP_CharacterEditor.SliderLeg` _widget) _proportions_lowerrightarmlength))

(event `LeaveEditor`
  (set `self.bShowMouseCursor` false)
  (`WidgetBlueprintLibrary.SetInputMode_GameOnly` self)
  (`GameplayStatics.OpenLevel` "PerlinNoise"))

(fn `UserConstructionScript`)