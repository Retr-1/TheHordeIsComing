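; BP_Lightbulb is a lightbulb actor whose light can be switched on and off.
; TurnOn and TurnOff set the IsOn flag and show or hide the Light component to match.
; Toggle reads IsOn and calls the opposite function.
; The event graph and construction script are empty, so switching relies on calls to these functions.
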(event `self.ReceiveBeginPlay`)

(event `self.ReceiveTick`
  (params (DeltaSeconds :type "Float (single-precision)")))

(fn `Toggle`
  (if (`self.IsOn`)
    (`self.TurnOff`)
    (else
      (`self.TurnOn`))))

(fn `TurnOff`
  (set `self.IsOn` false)
  (`SceneComponent.SetVisibility` (`self.Light`) false false))

(fn `TurnOn`
  (set `self.IsOn` true)
  (`SceneComponent.SetVisibility` (`self.Light`) true false))

(fn `UserConstructionScript`)