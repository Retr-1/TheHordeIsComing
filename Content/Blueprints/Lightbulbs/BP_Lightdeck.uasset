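; BP_Lightdeck is a deck of BP_Lightbulb child actors that shows a random on/off pattern, changing on a looping timer.
; On BeginPlay it gathers the bulbs from its root's child components and starts the timer, which also prints a separately rolled random number.
; SetState treats an integer as a bitmask, turning bulbs on for clear bits and off for set bits.
; ConstructDeck, which builds a bar and spawns bulbs, is not called here.
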(event `self.ReceiveBeginPlay`
  (`self.InitFromViewport`)
  (`KismetSystemLibrary.K2_SetTimerDelegate` (delegate `CustomEvent`) 2.0 true))

(event `CustomEvent`
  (bind _returnvalue (`KismetMathLibrary.RandomInteger` (`self.GetMaxMask`)))
  (`self.SetState` _returnvalue)
  (`KismetSystemLibrary.PrintString` (`KismetStringLibrary.Conv_IntToString` _returnvalue)))

(fn `AreAllActive`
  (returns (AreAllActive :type Boolean))
  (return (== (`self.CurrentState`) (`self.GetMaxMask`))))

(fn `ConstructDeck`
  (bind _returnvalue (`AddComponent|NODE_AddStaticMeshComponent-0` :`RelativeTransform` (`KismetMathLibrary.MakeTransform` (0.0 0.0 0.0) (struct) (`KismetMathLibrary.MakeVector` (* (`self.NumberOfBulbs`) (`self.BulbWidth`)) 0.2 0.2))))
  (`StaticMeshComponent.SetStaticMesh` _returnvalue "/Engine/BasicShapes/Cube.Cube")
  (for _ (range (`self.NumberOfBulbs`))
    (`|SpawnActorFromClass` "/Game/Blueprints/Lightbulbs/BP_Lightbulb.BP_Lightbulb_C" (`KismetMathLibrary.MakeTransform` (0.0 0.0 0.0)) "Undefined" "MultiplyWithRoot" null null)))

(fn `GetMaxMask`
  (returns (Mask :type Integer))
  (return (`KismetMathLibrary.FTrunc` (`KismetMathLibrary.MultiplyMultiply_FloatFloat` 2.0 (`KismetMathLibrary.Conv_IntToDouble` (`KismetArrayLibrary.Array_Length` (`self.Bulbs`)))))))

(fn `InitFromViewport`
  (for _array_element (`SceneComponent.GetChildrenComponents` (`self.DefaultSceneRoot`) false)
    (bind _aschild_actor_component (cast `ChildActorComponent` _array_element))
    (bind _asbp_lightbulb (cast `/Game/Blueprints/Lightbulbs/BP_Lightbulb` (`ChildActorComponent.ChildActor` _aschild_actor_component)))
    (`KismetArrayLibrary.Array_Add` (`self.Bulbs`) _asbp_lightbulb)))

(fn `SetState`
  (params (Mask :type Integer))
  (locals (MaskVar :type Integer))
  (bind _output_get (set `self.CurrentState` Mask))
  (set `local.MaskVar` _output_get)
  (for _array_element (`self.Bulbs`)
    (if (== (`KismetMathLibrary.And_IntInt` (`local.MaskVar`) 1) 0)
      (`/Game/Blueprints/Lightbulbs/BP_Lightbulb.TurnOn` _array_element)
      (else
        (`/Game/Blueprints/Lightbulbs/BP_Lightbulb.TurnOff` _array_element)))
    (set `local.MaskVar` (/ (`local.MaskVar`) 2))))

(fn `UserConstructionScript`)