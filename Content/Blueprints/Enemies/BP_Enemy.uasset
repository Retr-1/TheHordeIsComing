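; Enemy pawn that hunts players or buildables and reports its removal to the game mode.
; BeginPlay randomly picks a targeting mode: nearest player, nearest buildable, or switch.
; Tick re-issues AI MoveTo, falling back to players without targets; switch mode chases close players, otherwise the buildable nearest world origin.
; EndPlay decrements BP_BaseMode's enemy count and starts the exploring phase when none remain.
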(event `self.ReceiveBeginPlay`
  (set `self.Target` (`KismetArrayLibrary.Array_Random` (`|MakeArray` (`self.PlayerTag`) (`self.Buildable Tag`) (`self.SwitchTarget`)))))

(event `self.ReceiveTick`
  (params (DeltaSeconds :type "Float (single-precision)"))
  (bind _returnvalue (`CharacterMovementComponent.GetLastUpdateLocation` (`self.CharacterMovement`)))
  (if (!= (`self.Target`) (`self.SwitchTarget`))
    (bind _outactors (`GameplayStatics.GetAllActorsWithTag` (`self.Target`)))
    (if (`KismetArrayLibrary.Array_IsEmpty` _outactors)
      (bind _outactors_2 (`GameplayStatics.GetAllActorsWithTag` (`self.PlayerTag`)))
      (`|AIMoveTo` self (0.0 0.0 0.0) (`.ReturnValue` (`GameplayStatics.FindNearestActor` _returnvalue _outactors_2)))
      (else
        (`|AIMoveTo` self (0.0 0.0 0.0) (`.ReturnValue` (`GameplayStatics.FindNearestActor` _returnvalue _outactors)) 5.0 true)))
    (else
      (bind _outactors_3 (`GameplayStatics.GetAllActorsWithTag` (`self.PlayerTag`)))
      (bind (_distance _returnvalue_2) (`GameplayStatics.FindNearestActor` (`CharacterMovementComponent.GetLastUpdateLocation` (`self.CharacterMovement`)) _outactors_3))
      (if (<= _distance 1000.0)
        (`|AIMoveTo` self (0.0 0.0 0.0) _returnvalue_2)
        (else
          (bind _outactors_4 (`GameplayStatics.GetAllActorsWithTag` (`self.Buildable Tag`)))
          (`|AIMoveTo` self (0.0 0.0 0.0) (`.ReturnValue` (`GameplayStatics.FindNearestActor` (0.0 0.0 0.0) _outactors_4))))))))

(event `self.ReceiveEndPlay`
  (params (EndPlayReason :type "EEndPlayReason Enum" :default "Destroyed"))
  (bind _asbp_base_mode (cast `/Game/Blueprints/BP_BaseMode` (`GameplayStatics.GetGameMode`)))
  (bind _numberofenemies (`/Game/Blueprints/BP_BaseMode.NumberOfEnemies` _asbp_base_mode))
  (set `/Game/Blueprints/BP_BaseMode.NumberOfEnemies` (- _numberofenemies 1) _asbp_base_mode)
  (if (<= _numberofenemies 0)
    (`/Game/Blueprints/BP_BaseMode.ExploringPhaseStart` _asbp_base_mode)))

(fn `UserConstructionScript`)