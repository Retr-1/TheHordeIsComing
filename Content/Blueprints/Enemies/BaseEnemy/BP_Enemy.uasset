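; Base enemy that hunts the player or buildables, picking a random targeting mode at spawn.
; Tick issues AIMoveTo toward the nearest tagged actor or player fallback; switch mode prefers the player when close, otherwise buildables.
; On arrival, it stops moving and, after a windup, damages players and buildables in a sphere overlap.
; Destruction grants XP and drops a coin; EndPlay decrements BP_BaseMode's count for spawned enemies, starting exploration at zero.
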(event `self.ReceiveBeginPlay`
  (set `self.Target` (`KismetArrayLibrary.Array_Random` (`|MakeArray` (`self.PlayerTag`) (`self.Buildable Tag`) (`self.SwitchTarget`)))))

(event `self.ReceiveTick`
  (params (DeltaSeconds :type "Float (single-precision)"))
  (bind _returnvalue (`GameplayStatics.GetPlayerPawn` 0))
  (if (!= (`self.Target`) (`self.SwitchTarget`))
    (bind _outactors (`GameplayStatics.GetAllActorsWithTag` (`self.Target`)))
    (if (`KismetArrayLibrary.Array_IsEmpty` _outactors)
      (`|AIMoveTo` self (0.0 0.0 0.0) (`GameplayStatics.GetPlayerPawn` 0) 200.0
        (:`OnSuccess`
          _))
      (else
        (`|AIMoveTo` self (0.0 0.0 0.0) (`.ReturnValue` (`GameplayStatics.FindNearestActor` (`CharacterMovementComponent.GetLastUpdateLocation` (`self.CharacterMovement`)) _outactors)) 200.0
          (:`OnSuccess`
            _))))
    (elif (<= (`self.GetDistanceTo` self _returnvalue) 1000.0)
      (`|AIMoveTo` self (0.0 0.0 0.0) _returnvalue 200.0
        (:`OnSuccess`
          _))
      (else
        (bind _outactors_2 (`GameplayStatics.GetAllActorsWithTag` (`self.Buildable Tag`)))
        (`|AIMoveTo` self (0.0 0.0 0.0) (`.ReturnValue` (`GameplayStatics.FindNearestActor` (`CharacterMovementComponent.GetLastUpdateLocation` (`self.CharacterMovement`)) _outactors_2)) 200.0
          (:`OnSuccess`
            _)))))
  (`self.Attack` null))

(event `self.ReceiveEndPlay`
  (params (EndPlayReason :type "EEndPlayReason Enum" :default "Destroyed"))
  (if (`self.ActorHasTag` (`self.EnemySpawned`))
    (bind _asbp_base_mode (cast `/Game/Blueprints/BP_BaseMode` (`GameplayStatics.GetGameMode`)))
    (bind _numberofenemies (`/Game/Blueprints/BP_BaseMode.NumberOfEnemies` _asbp_base_mode))
    (set `/Game/Blueprints/BP_BaseMode.NumberOfEnemies` (- _numberofenemies 1) _asbp_base_mode)
    (if (<= _numberofenemies 0)
      (`/Game/Blueprints/BP_BaseMode.ExploringPhaseStart` _asbp_base_mode))))

(event `Attack`
  (params (Target :type "Actor Object Reference"))
  (`AIController.K2_SetFocus` (`AIBlueprintHelperLibrary.GetAIController` self) Target)
  (set `self.IsAttacking` true)
  (`CharacterMovementComponent.DisableMovement` (`self.CharacterMovement`))
  (`KismetSystemLibrary.Delay` 1.5)
  (bind _outactors (`KismetSystemLibrary.SphereOverlapActors` (`SceneComponent.K2_GetComponentLocation` (`self.Arrow1`)) 150.0 (`self.Object Types`)))
  (for _array_element _outactors
    (`self.Deal Damage` _array_element))
  (`KismetSystemLibrary.Delay` 0.5)
  (set `self.IsAttacking` false)
  (`CharacterMovementComponent.SetMovementMode` (`self.CharacterMovement`) "MOVE_Walking" 0))

(event `Deal Damage`
  (params (Targeting :type "Actor Object Reference"))
  (if (`self.ActorHasTag` Targeting "Player")
    (`GameplayStatics.ApplyDamage` Targeting (`self.Damage`))
    (elif (`self.ActorHasTag` Targeting "Buildable")
      (`GameplayStatics.ApplyDamage` Targeting (`self.Damage`)))))

(event `self.ReceiveDestroyed`
  (bind _returnvalue_location (`KismetMathLibrary.BreakTransform` (`self.GetTransform`)))
  (bind _asbp_base_character (cast `/Game/Blueprints/BP_BaseCharacter_Noro` (`GameplayStatics.GetPlayerCharacter` 0)))
  (`/Game/Blueprints/BP_BaseCharacter_Noro.Add Xp` _asbp_base_character 1.0)
  (`|SpawnActorFromClass` "/Game/Assets/Mesh/Drops/Coin/BP_Coin.BP_Coin_C" (`KismetMathLibrary.MakeTransform` _returnvalue_location) "Undefined" "MultiplyWithRoot" null null))

(fn `UserConstructionScript`)