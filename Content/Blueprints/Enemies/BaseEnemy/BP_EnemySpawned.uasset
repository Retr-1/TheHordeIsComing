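; BP_EnemySpawned is an enemy variant, apparently for spawned enemies, with only a few overrides on its parent's logic.
; Its construction script runs the parent's and then sets a fixed maximum distance.
; SetTarget picks the target at random from the player, crystal camera and switch target tags.
; The event graph holds only disabled placeholder events.
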(fn `SetTarget`
  (set `self.Target` (`KismetArrayLibrary.Array_Random` (`|MakeArray` (`self.PlayerTag`) (`self.CrystalCamera Tag`) (`self.SwitchTarget`)))))

(fn `UserConstructionScript`
  (`parent.UserConstructionScript`)
  (set `self.MaxDistance` 6000.0))