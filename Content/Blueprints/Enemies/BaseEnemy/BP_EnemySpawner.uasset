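; BP_EnemySpawner is an enemy spawner that creates enemies from a queue of classes at its own transform.
; AddEnemyToQueue appends a class and immediately calls SpawnEnemy.
; SpawnEnemy spawns the first queued class, tags it as a spawned enemy, removes it from the queue and sets a one-second timer by function name.
; It returns whether an enemy was queued to spawn.
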(fn `AddEnemyToQueue`
  (params (EnemyClass :type "/Game/Blueprints/Enemies/BaseEnemy/BP_Enemy Class Reference"))
  (`KismetArrayLibrary.Array_Add` (`self.EnemyQueue`) EnemyClass)
  (`self.SpawnEnemy`))

(fn `SpawnEnemy`
  (returns (Success :type Boolean))
  (if (`KismetArrayLibrary.Array_IsValidIndex` (`self.EnemyQueue`))
    (bind _returnvalue (`|SpawnActorFromClass` (`|GetArrayItem` (`self.EnemyQueue`)) (`self.GetTransform`) "Undefined" "MultiplyWithRoot" null null))
    (set `Actor.Tags` (`|MakeArray` "Enemy" "EnemySpawned" :!type "Name") _returnvalue)
    (`KismetArrayLibrary.Array_Remove` (`self.EnemyQueue`))
    (`KismetSystemLibrary.K2_SetTimer` null "" 1.0)
    (return true)
    (else
      (return false))))

(fn `UserConstructionScript`)