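; Puzzle room where flipping levers toggles lights on a lightdeck until all are active, which destroys the barrier and marks the room solved.
; On BeginPlay the deck starts at its maximum state, and each generated random bitmask pattern has a coin-flip chance to scramble it, keeping the puzzle solvable by construction.
; Six child-actor levers receive index IDs, and their change events toggle the matching pattern and check the solution.
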(event `self.ReceiveBeginPlay`
  (`parent.ReceiveBeginPlay`)
  (bind _asbp_lightdeck (cast `/Game/Blueprints/Structures/Lightbulbs/BP_Lightdeck` (`ChildActorComponent.ChildActor` (`self.BP_Lightdeck`))))
  (bind _output_get (set `self.Lightdeck` _asbp_lightdeck))
  (`/Game/Blueprints/Structures/Lightbulbs/BP_Lightdeck.SetState` _output_get (`/Game/Blueprints/Structures/Lightbulbs/BP_Lightdeck.GetMaxState` _output_get))
  (`self.InitializePatterns`)
  (for (_array_element _array_index) (`|MakeArray` (`self.BP_Lever`) (`self.BP_Lever1`) (`self.BP_Lever2`) (`self.BP_Lever3`) (`self.BP_Lever4`) (`self.BP_Lever5`))
    (bind _asbp_lever (cast `/Game/Blueprints/Structures/BP_Lever` (`ChildActorComponent.ChildActor` _array_element)))
    (set `/Game/Blueprints/Structures/BP_Lever.ID` _array_index _asbp_lever)
    (add `/Game/Blueprints/Structures/BP_Lever.ChangedState` _asbp_lever (delegate `LeverChangedState`))))

(event `LeverChangedState`
  (params (Instigator :type "/Game/Blueprints/Structures/BP_Lever Object Reference"))
  (bind _output (`|GetArrayItem` (`self.Patterns`) (`/Game/Blueprints/Structures/BP_Lever.ID` Instigator)))
  (`/Game/Blueprints/Structures/Lightbulbs/BP_Lightdeck.Toggle` (`self.Lightdeck`) _output)
  (`self.VerifySolution`)
  (`KismetSystemLibrary.PrintString` (`KismetStringLibrary.Conv_IntToString` _output)))

(fn `GetLootTableID`
  (returns (LootTableID :type Name))
  (return "Basic"))

(fn `InitializePatterns`
  (locals (GeneratedMask :type Integer :default 0))
  (for _ (range (`self.LeverCount`))
    (bind _output_get (set `local.GeneratedMask` (`KismetMathLibrary.RandomIntegerInRange` 1 (`/Game/Blueprints/Structures/Lightbulbs/BP_Lightdeck.GetMaxState` (`self.Lightdeck`)))))
    (`KismetArrayLibrary.Array_Add` (`self.Patterns`) _output_get)
    (if (`KismetMathLibrary.RandomBool`)
      (`/Game/Blueprints/Structures/Lightbulbs/BP_Lightdeck.Toggle` (`self.Lightdeck`) (`local.GeneratedMask`)))))

(fn `UserConstructionScript`
  (`parent.UserConstructionScript`))

(fn `VerifySolution`
  (if (`self.GetIsSolved`)
    _
    (elif (`/Game/Blueprints/Structures/Lightbulbs/BP_Lightdeck.AreAllActive` (`self.Lightdeck`))
      (`KismetSystemLibrary.PrintString` "YAAY YOU SOLVED IT!!!")
      (`self.DestroyBarrier`)
      (`ActorComponent.K2_DestroyComponent` (`self.BP_Lightdeck`))
      (`self.SetIsSolved` true))))