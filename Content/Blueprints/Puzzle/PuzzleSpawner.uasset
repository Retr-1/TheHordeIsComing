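; PuzzleSpawner is a placed actor that builds a puzzle entrance and its linked room at game start.
; On BeginPlay it spawns EntranceClass scaled up at its own location and RoomClass, also scaled, at a fixed point far below the world origin.
; It then cross-links them, giving the entrance the room's player spawn point and the room's leave teleporter the entrance's exit location.
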(event `self.ReceiveBeginPlay`
  (bind _returnvalue (`|SpawnActorFromClass` (`self.EnteranceClass`) (`KismetMathLibrary.MakeTransform` (`self.K2_GetActorLocation`) (struct) (6.0 6.0 6.0)) "Undefined" "MultiplyWithRoot" null null))
  (set `self.Enterance` _returnvalue)
  (bind _returnvalue_2 (`|SpawnActorFromClass` (`self.RoomClass`) (`KismetMathLibrary.MakeTransform` (0.0 0.0 -10000.0) (struct) (7.0 7.0 7.0)) "Undefined" "MultiplyWithRoot" null null))
  (set `self.Room` _returnvalue_2)
  (`/Game/Blueprints/Puzzle/PuzzleEnterance.SetRoomPlayerSpawnLocation` (`self.Enterance`) (`SceneComponent.K2_GetComponentLocation` (`/Game/Blueprints/Puzzle/PuzzleRoom.PlayerSpawnPoint` (`self.Room`))))
  (`/Game/Blueprints/Puzzle/PuzzleRoom.SetLeaveTeleporterLocation` (`self.Room`) (`SceneComponent.K2_GetComponentLocation` (`/Game/Blueprints/Puzzle/PuzzleEnterance.PlayerLeaveLocation` (`self.Enterance`)))))

(fn `UserConstructionScript`)