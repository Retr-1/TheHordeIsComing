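; Build-mode component that lets the player preview, rotate, place and destroy buildables loaded from DT_BuildParts.
; In build mode, Tick camera-traces to position a ghost mesh, created through a DoOnce that resets on selection change or range crossing to refresh its valid/too-far material.
; Mouse wheel picks the part, rotation steps yaw 90 degrees, and placing spawns its actor on an in-range trace hit, then exits.
; Destroying removes traced "Buildable"-tagged actors.
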(event `DistanceCheck`
  (bind _build_preview_transform_location (`KismetMathLibrary.BreakTransform` (`self.Build Preview Transform`)))
  (bind _maxbuilddistance (`self.MaxBuildDistance`))
  (bind _returnvalue_location (`KismetMathLibrary.BreakTransform` (`SceneComponent.K2_GetComponentToWorld` (`self.Camera`))))
  (bind _returnvalue (`KismetMathLibrary.Vector_Distance` _returnvalue_location _build_preview_transform_location))
  (if (not (== (> _returnvalue _maxbuilddistance) (> (`self.RayhitDistance`) _maxbuilddistance)))
    (set `self.RayhitDistance` _returnvalue)
    (bind _preview_mesh (`self.Preview Mesh`)
      (:`then`
        (`StaticMeshComponent.SetStaticMesh` _preview_mesh null)
        (set `self.Preview Mesh` null)
        (`self.Reset Build Mode`))
      (:`else`))))

(event `self.ReceiveBeginPlay`
  (bind _asbp_base_character (cast `/Game/Blueprints/BP_BaseCharacter_Noro` (`GameplayStatics.GetPlayerCharacter` 0)))
  (set `self.Player BP` _asbp_base_character)
  (set `self.Camera` (`/Game/Blueprints/BP_BaseCharacter_Noro.Camera` _asbp_base_character))
  (bind _outrownames (`DataTableFunctionLibrary.GetDataTableRowNames` "/Game/Blueprints/DT_BuildParts.DT_BuildParts"))
  (for _array_element _outrownames
    (bind _returnvalue (`|GetDataTableRow` "/Game/Blueprints/DT_BuildParts.DT_BuildParts" _array_element)
      (:`then`
        (`KismetArrayLibrary.Array_Add` (`self.DT_Buildables`) _returnvalue)))))

(event `self.ReceiveTick`
  (params (DeltaSeconds :type "Float (single-precision)"))
  (if (`self.InBuildMode`)
    (`self.Preview Loop`)))

(event `Preview Loop`
  (bind _preview_mesh (`self.Preview Mesh`))
  (bind (_returnvalue_location _returnvalue_rotation) (`KismetMathLibrary.BreakTransform` (`SceneComponent.K2_GetComponentToWorld` (`self.Camera`))))
  (`self.DistanceCheck`)
  (bind (_outhit _returnvalue) (`KismetSystemLibrary.LineTraceSingle` _returnvalue_location (+ _returnvalue_location (* (`KismetMathLibrary.GetForwardVector` _returnvalue_rotation) 2000.0)) "TraceTypeQuery1"))
  (if _returnvalue
    (`|ExecutionSequence`
      (:`then_0`
        (`/Engine/EditorBlueprintResources/StandardMacros.DoOnce` false :!label _label
          (:`Completed`
            (bind _returnvalue_2 (`|AddComponentByClass` (`self.Player BP`) "/Script/Engine.StaticMeshComponent" false (`self.Build Preview Transform`)))
            (bind _output_get (set `self.Preview Mesh` _returnvalue_2))
            (`StaticMeshComponent.SetStaticMesh` _output_get (`.Mesh_5_40A5556C4F058EA5912480A8693D8804` (break `/Game/Blueprints/S_BuildParts` (`|GetArrayItem` (`self.DT_Buildables`) (`self.buildable index`)))))
            (for _index (range (`PrimitiveComponent.GetNumMaterials` _preview_mesh))
              (if (<= (`self.RayhitDistance`) (`self.MaxBuildDistance`))
                (`PrimitiveComponent.SetMaterial` _preview_mesh _index "/Game/Assets/Materials/M_BuildPreview.M_BuildPreview")
                (else
                  (`PrimitiveComponent.SetMaterial` _preview_mesh _index "/Game/Assets/Materials/M_PreviewTooFar.M_PreviewTooFar"))))
            (`PrimitiveComponent.SetCollisionEnabled` _preview_mesh "NoCollision"))))
      (:`then_1`
        (bind _output_get_2 (set `self.Build Preview Transform` (`KismetMathLibrary.MakeTransform` (`.Location` (`GameplayStatics.BreakHitResult` _outhit)) (`KismetMathLibrary.MakeRotator` 0.0 0.0 (`KismetMathLibrary.Conv_IntToDouble` (`self.BuildRotation`))) (0.3 0.3 0.3))))
        (`SceneComponent.K2_SetWorldTransform` (`self.Preview Mesh`) _output_get_2 false false)))
    (else
      (bind _preview_mesh_2 (`self.Preview Mesh`)
        (:`then`
          (`StaticMeshComponent.SetStaticMesh` _preview_mesh_2 null)
          (set `self.Preview Mesh` null)
          (`self.Reset Build Mode`))
        (:`else`)))))

(event `Reset Build Mode`
  (goto _label :!via `Reset`))

(event `EnhancedInput|/Game/Inputs/IA_Build`
  (params (ActionValue :type Boolean) (ElapsedSeconds :type "Float (double-precision)") (TriggeredSeconds :type "Float (double-precision)") (InputAction :type "InputAction Object Reference" :default "/Game/Inputs/IA_Build.IA_Build"))
  (:`Started`
    (if (not (`self.InBuildMode`))
      (set `self.InBuildMode` true)
      (else
        (set `self.InBuildMode` false :!label _label_2)
        (bind _preview_mesh (`self.Preview Mesh`)
          (:`then`
            (`StaticMeshComponent.SetStaticMesh` _preview_mesh null)
            (set `self.Preview Mesh` null)
            (`self.Reset Build Mode`))
          (:`else`))))))

(event `Stop Build Mode`
  (goto _label_2))

(event `EnhancedInput|/Game/Inputs/IA_PlaceBuild`
  (params (ActionValue :type Boolean) (ElapsedSeconds :type "Float (double-precision)") (TriggeredSeconds :type "Float (double-precision)") (InputAction :type "InputAction Object Reference" :default "/Game/Inputs/IA_PlaceBuild.IA_PlaceBuild"))
  (bind (_returnvalue_location _returnvalue_rotation) (`KismetMathLibrary.BreakTransform` (`SceneComponent.K2_GetComponentToWorld` (`self.Camera`))))
  (:`Triggered`
    (if (`self.InBuildMode`)
      (bind (_outhit _returnvalue) (`KismetSystemLibrary.LineTraceSingle` _returnvalue_location (+ _returnvalue_location (* (`KismetMathLibrary.GetForwardVector` _returnvalue_rotation) (`self.MaxBuildDistance`))) "TraceTypeQuery1"))
      (if _returnvalue
        (`|SpawnActorFromClass` (`.Actor_9_E7AD1CBD46564CA72741B893DB4B4088` (break `/Game/Blueprints/S_BuildParts` (`|GetArrayItem` (`self.DT_Buildables`) (`self.buildable index`)))) (`self.Build Preview Transform`) "AlwaysSpawn" "MultiplyWithRoot" null null)
        (`self.Stop Build Mode`)))))

(event `Key|MouseScrollUp`
  (params (Key :type "Key Structure"))
  (:`Pressed`
    (set `self.buildable index` (`KismetMathLibrary.Clamp` (+ (`self.buildable index`) 1) 0 (- (`KismetArrayLibrary.Array_Length` (`self.DT_Buildables`)) 1)))
    (bind _preview_mesh (`self.Preview Mesh` :!label _label_3)
      (:`then`
        (`StaticMeshComponent.SetStaticMesh` _preview_mesh null)
        (set `self.Preview Mesh` null)
        (`self.Reset Build Mode`))
      (:`else`))))

(event `Key|MouseScrollDown`
  (params (Key :type "Key Structure"))
  (:`Pressed`
    (set `self.buildable index` (`KismetMathLibrary.Clamp` (- (`self.buildable index`) 1) 0 (- (`KismetArrayLibrary.Array_Length` (`self.DT_Buildables`)) 1)))
    (goto _label_3)))

(event `EnhancedInput|/Game/Inputs/IA_DestroyBuild`
  (params (ActionValue :type Boolean) (ElapsedSeconds :type "Float (double-precision)") (TriggeredSeconds :type "Float (double-precision)") (InputAction :type "InputAction Object Reference" :default "/Game/Inputs/IA_DestroyBuild.IA_DestroyBuild"))
  (bind (_returnvalue_location _returnvalue_rotation) (`KismetMathLibrary.BreakTransform` (`SceneComponent.K2_GetComponentToWorld` (`self.Camera`))))
  (:`Started`
    (bind (_outhit _returnvalue) (`KismetSystemLibrary.LineTraceSingle` _returnvalue_location (+ _returnvalue_location (* (`KismetMathLibrary.GetForwardVector` _returnvalue_rotation) 700.0)) "TraceTypeQuery1"))
    (if _returnvalue
      (bind (_bblockinghit _binitialoverlap _time _distance _location _impactpoint _normal _impactnormal _physmat _hitactor) (`GameplayStatics.BreakHitResult` _outhit))
      (if (`Actor.ActorHasTag` _hitactor "Buildable")
        (`Actor.K2_DestroyActor` _hitactor)))))

(event `EnhancedInput|/Game/Inputs/IA_RotateBuild`
  (params (ActionValue :type Boolean) (ElapsedSeconds :type "Float (double-precision)") (TriggeredSeconds :type "Float (double-precision)") (InputAction :type "InputAction Object Reference" :default "/Game/Inputs/IA_RotateBuild.IA_RotateBuild"))
  (:`Started`
    (if (`self.InBuildMode`)
      (set `self.BuildRotation` (mod (+ (`self.BuildRotation`) 90) 360)))))