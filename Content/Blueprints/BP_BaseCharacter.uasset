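; Base player character with movement, inventory, crafting, building, resource harvesting, shooting, XP and skill upgrades.
; Each tick a camera trace drives pickup and interact hints, while a world-height check drains oxygen, then health.
; The active hotbar item, resolved through data tables, sets the held mesh, harvesting tool and build mode.
; On death it destroys itself and asks the game mode to respawn it at the nearest spawn point.
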(event `self.ReceiveBeginPlay`
  (bind _returnvalue (`|CreateWidget` "/Game/Blueprints/UserInterface/WB_ItemFocusInfo.WB_ItemFocusInfo_C" null 0 null))
  (bind _output_get (set `self.ItemFocusWidget` _returnvalue))
  (`UserWidget.AddToViewport` _output_get 0)
  (bind _returnvalue_2 (`|CreateWidget` "/Game/Blueprints/UserInterface/WBP_Inventory.WBP_Inventory_C" null (`self.BPC_InventoryComponent`)))
  (`UserWidget.AddToViewport` _returnvalue_2 0)
  (`Widget.SetVisibility` _returnvalue_2 "Hidden")
  (set `self.InventoryWidget` _returnvalue_2)
  (bind _returnvalue_3 (`|CreateWidget` "/Game/Blueprints/UserInterface/WB_PlayerHealthBar.WB_PlayerHealthBar_C"))
  (set `self.HealthBarWidget` _returnvalue_3)
  (`UserWidget.AddToViewport` _returnvalue_3 0)
  (`/Game/Blueprints/UserInterface/WB_PlayerHealthBar.Initialize` _returnvalue_3 self)
  (bind _asbp_game_instance (cast `/Game/Blueprints/BP_GameInstance` (`GameplayStatics.GetGameInstance`)))
  (set `self.BodyProportions` (`/Game/Blueprints/BP_GameInstance.Proportions` _asbp_game_instance))
  (bind _returnvalue_4 (`|CreateWidget` "/Game/Blueprints/UserInterface/WBP_InteractTooltip.WBP_InteractTooltip_C"))
  (bind _output_get_2 (set `self.InteractTooltipWidget` _returnvalue_4))
  (`UserWidget.AddToViewport` _output_get_2 0)
  (`self.CoinUpdate` 0)
  (`self.Set Active Hotbar Index` 0)
  (add `/Game/Blueprints/Components/BPC_InventoryComponent.InventoryChanged` (`self.BPC_InventoryComponent`) (delegate `InventoryChangedEvent`))
  (set `self.LastPosition` (`self.K2_GetActorLocation`))
  (`KismetSystemLibrary.Delay` 0.3)
  (set `self.Spawned` true))

(event `self.ReceiveTick`
  (params (DeltaSeconds :type "Float (single-precision)"))
  (bind _returnvalue (`self.K2_GetActorLocation`))
  (`self.ResolveHoverOnActors`)
  (`self.Resolve Oxygen`)
  (set `self.DistanceWalked` (+ (`self.DistanceWalked`) (`KismetMathLibrary.Vector_Distance` (`self.LastPosition`) _returnvalue)))
  (set `self.LastPosition` _returnvalue))

(event `InventoryChangedEvent`
  (params (Instigator :type "/Game/Blueprints/Components/BPC_InventoryComponent Object Reference"))
  (`self.Set Active Hotbar Index` (`/Game/Blueprints/Components/BPC_InventoryComponent.ActiveHotbarIndex` (`self.BPC_InventoryComponent`))))

(event `EnhancedInput|/Game/Inputs/IA_MoveForward`
  (params (ActionValue :type "Float (double-precision)") (ElapsedSeconds :type "Float (double-precision)") (TriggeredSeconds :type "Float (double-precision)") (InputAction :type "InputAction Object Reference" :default "/Game/Inputs/IA_MoveForward.IA_MoveForward"))
  (bind (_returnvalue_roll _returnvalue_pitch _returnvalue_yaw) (`KismetMathLibrary.BreakRotator` (`self.GetControlRotation`)))
  (:`Triggered`
    (`self.AddMovementInput` (`KismetMathLibrary.GetForwardVector` (`KismetMathLibrary.MakeRotator` 0.0 0.0 _returnvalue_yaw)) ActionValue)))

(event `EnhancedInput|/Game/Inputs/IA_MoveRight`
  (params (ActionValue :type "Float (double-precision)") (ElapsedSeconds :type "Float (double-precision)") (TriggeredSeconds :type "Float (double-precision)") (InputAction :type "InputAction Object Reference" :default "/Game/Inputs/IA_MoveRight.IA_MoveRight"))
  (bind (_returnvalue_roll _returnvalue_pitch _returnvalue_yaw) (`KismetMathLibrary.BreakRotator` (`self.GetControlRotation`)))
  (:`Triggered`
    (`self.AddMovementInput` (`KismetMathLibrary.GetRightVector` (`KismetMathLibrary.MakeRotator` 0.0 0.0 _returnvalue_yaw)) ActionValue)))

(event `EnhancedInput|/Game/Inputs/IA_Jump`
  (params (ActionValue :type Boolean) (ElapsedSeconds :type "Float (double-precision)") (TriggeredSeconds :type "Float (double-precision)") (InputAction :type "InputAction Object Reference" :default "/Game/Inputs/IA_Jump.IA_Jump"))
  (:`Triggered`
    (if (not (`self.IsJumping`))
      (`self.Jump`)))
  (:`Canceled`
    (`self.StopJumping` :!label _label))
  (:`Completed`
    (goto _label)))

(event `self.OnJumped`
  (set `self.IsJumping` true))

(event `self.OnLanded`
  (params (Hit :type "HitResult Structure (by ref)"))
  (`KismetSystemLibrary.Delay` 0.8)
  (set `self.IsJumping` false))

(event `EnhancedInput|/Game/Inputs/IA_Sprint`
  (params (ActionValue :type Boolean) (ElapsedSeconds :type "Float (double-precision)") (TriggeredSeconds :type "Float (double-precision)") (InputAction :type "InputAction Object Reference" :default "/Game/Inputs/IA_Sprint.IA_Sprint"))
  (:`Triggered`
    (`self.Sprint`))
  (:`Completed`
    (`self.StopSprint`)))

(event `EnhancedInput|/Game/Inputs/IA_Interact`
  (params (ActionValue :type Boolean) (ElapsedSeconds :type "Float (double-precision)") (TriggeredSeconds :type "Float (double-precision)") (InputAction :type "InputAction Object Reference" :default "/Game/Inputs/IA_Interact.IA_Interact"))
  (:`Started`
    (`self.Resolve Interact`)))

(event `EnhancedInput|/Game/Inputs/IA_FireBullet`
  (params (ActionValue :type Boolean) (ElapsedSeconds :type "Float (double-precision)") (TriggeredSeconds :type "Float (double-precision)") (InputAction :type "InputAction Object Reference" :default "/Game/Inputs/IA_FireBullet.IA_FireBullet"))
  (bind _camera (`self.Camera`))
  (:`Triggered`
    (`|SpawnActorFromClass` "/Game/Blueprints/BP_Bullet.BP_Bullet_C" (`KismetMathLibrary.MakeTransform` (+ (`SceneComponent.K2_GetComponentLocation` _camera) (* (`SceneComponent.GetForwardVector` _camera) 100.0)) (`SceneComponent.K2_GetComponentRotation` _camera)) "Undefined" "MultiplyWithRoot" null null)))

(event `EnhancedInput|/Game/Inputs/Hitting`
  (params (ActionValue :type Boolean) (ElapsedSeconds :type "Float (double-precision)") (TriggeredSeconds :type "Float (double-precision)") (InputAction :type "InputAction Object Reference" :default "/Game/Inputs/Hitting.Hitting"))
  (:`Triggered`
    (`self.InitializeAttack`)))

(event `EnhancedInput|/Game/Inputs/IA_OpenInventory`
  (params (ActionValue :type Boolean) (ElapsedSeconds :type "Float (double-precision)") (TriggeredSeconds :type "Float (double-precision)") (InputAction :type "InputAction Object Reference" :default "/Game/Inputs/IA_OpenInventory.IA_OpenInventory"))
  (bind _returnvalue (`GameplayStatics.GetPlayerController` 0))
  (bind _inventorywidget (`self.InventoryWidget`))
  (:`Triggered`
    (`/Engine/EditorBlueprintResources/StandardMacros.FlipFlop`
      (:`A`
        (`Widget.SetVisibility` _inventorywidget "Visible")
        (`/Game/Blueprints/UserInterface/WBP_Inventory.RefreshAllSlots` (`self.InventoryWidget`))
        (`WidgetBlueprintLibrary.SetInputMode_GameAndUIEx` _returnvalue null)
        (set `PlayerController.bShowMouseCursor` true _returnvalue))
      (:`B`
        (`Widget.SetVisibility` _inventorywidget "Hidden")
        (`WidgetBlueprintLibrary.SetInputMode_GameOnly` _returnvalue)
        (set `PlayerController.bShowMouseCursor` false _returnvalue)))))

(event `self.ReceiveAnyDamage`
  (params (Damage :type "Float (single-precision)") (DamageType :type "DamageType Object Reference") (InstigatedBy :type "Controller Object Reference") (DamageCauser :type "Actor Object Reference"))
  (bind _output_get (set `self.CurrentHealth` (- (`self.CurrentHealth`) Damage)))
  (`self.HealthUpdated` _output_get (`self.MaxHealth`))
  (if (<= _output_get 0.0)
    (`self.Death`)))

(event `Death`
  (`self.K2_DestroyActor`))

(event `self.ReceiveDestroyed`
  (bind _returnvalue_location (`KismetMathLibrary.BreakTransform` (`self.GetTransform`)))
  (bind _outactors (`GameplayStatics.GetAllActorsOfClass` "/Game/Blueprints/BP_SpawnPos.BP_SpawnPos_C"))
  (bind _asbp_base_mode (cast `/Game/Blueprints/BP_BaseMode` (`GameplayStatics.GetGameMode`)))
  (`/Game/Blueprints/BP_BaseMode.Respawn Player` _asbp_base_mode (`self.GetTransform` (`.ReturnValue` (`GameplayStatics.FindNearestActor` _returnvalue_location _outactors)))))

(event `EnhancedInput|/Game/Inputs/IA_OpenCrafting`
  (params (ActionValue :type Boolean) (ElapsedSeconds :type "Float (double-precision)") (TriggeredSeconds :type "Float (double-precision)") (InputAction :type "InputAction Object Reference" :default "/Game/Inputs/IA_OpenCrafting.IA_OpenCrafting"))
  (:`Triggered`
    (`/Game/Blueprints/Components/BPC_CraftingComponent.ToggleCraftingUIVisibility` (`self.BPC_CraftingComponent`))))

(event `EnhancedInput|/Game/Inputs/IA_OpenSkillTree`
  (params (ActionValue :type Boolean) (ElapsedSeconds :type "Float (double-precision)") (TriggeredSeconds :type "Float (double-precision)") (InputAction :type "InputAction Object Reference" :default "/Game/Inputs/IA_OpenSkillTree.IA_OpenSkillTree"))
  (bind _returnvalue (`GameplayStatics.GetPlayerController` 0))
  (bind _returnvalue_2 (`GameplayStatics.GetPlayerController` 0))
  (bind _skilltreewidget (`self.SkillTreeWidget`))
  (:`Started`
    (bind _skilltreewidget_2 (`self.SkillTreeWidget`)
      (:`then`
        (`Widget.RemoveFromParent` _skilltreewidget_2)
        (`self.Save Skill Tree`)
        (set `self.SkillTreeWidget` null)
        (set `PlayerController.bShowMouseCursor` false _returnvalue_2)
        (`WidgetBlueprintLibrary.SetInputMode_GameOnly` _returnvalue_2))
      (:`else`
        (bind _returnvalue_3 (`|CreateWidget` "/Game/Blueprints/UserInterface/SkillTree/WB_SkillTree.WB_SkillTree_C"))
        (bind _output_get (set `self.SkillTreeWidget` _returnvalue_3))
        (`UserWidget.AddToViewport` _output_get 0)
        (set `PlayerController.bShowMouseCursor` true _returnvalue)
        (`WidgetBlueprintLibrary.SetInputMode_GameAndUIEx` _returnvalue null)
        (set `/Game/Blueprints/UserInterface/SkillTree/WB_SkillTree.Player` self _skilltreewidget)
        (`/Game/Blueprints/UserInterface/SkillTree/WB_SkillTree.Initialize from player` _skilltreewidget)))))

(event `Add Xp`
  (params (Increment :type "Float (double-precision)"))
  (if (`self.Spawned`)
    (set `self.XP` (`KismetMathLibrary.FMin` (+ (`self.XP`) (* Increment (`self.XP multiplier`))) (`self.XP to lvl up`)))
    (set `self.KillCount` (+ (`self.KillCount`) 1))
    (if (>= (`self.XP`) (`self.XP to lvl up`))
      (`self.Lvl up`))))

(event `Get Skill`
  (params (Skill :type "/Game/Blueprints/UserInterface/SkillTree/ENUM_SkillTree Enum" :default "NewEnumerator0"))
  (set `self.SkillPoints` (- (`self.SkillPoints`) 1))
  (switch `/Game/Blueprints/UserInterface/SkillTree/ENUM_SkillTree` Skill
    (:`NewEnumerator0`
      (set `self.Damage` (* (`self.Damage`) 1.15) :!label _label_2))
    (:`NewEnumerator1`
      (goto _label_2))
    (:`NewEnumerator2`
      (goto _label_2))
    (:`NewEnumerator3`
      (goto _label_2))
    (:`NewEnumerator4`
      (goto _label_2))
    (:`NewEnumerator5`
      (bind _output_get (set `self.MaxHealth` (+ (`self.MaxHealth`) 20.0) :!label _label_3))
      (bind _output_get_2 (set `self.CurrentHealth` _output_get))
      (`self.HealthUpdated` _output_get_2 _output_get))
    (:`NewEnumerator6`
      (goto _label_3))
    (:`NewEnumerator7`
      (goto _label_3))
    (:`NewEnumerator13`
      (goto _label_3))
    (:`NewEnumerator8`
      (set `self.MaxOxygen` (* (`self.MaxOxygen`) 2.0)))
    (:`NewEnumerator9`
      (set `self.XP multiplier` (+ (`self.XP multiplier`) 1.0) :!label _label_4))
    (:`NewEnumerator10`
      (goto _label_4))
    (:`NewEnumerator11`
      (set `self.Coin multiplier` (+ (`self.Coin multiplier`) 1) :!label _label_5))
    (:`NewEnumerator12`
      (goto _label_5))
    (:`NewEnumerator14`
      (bind _output_get_3 (set `self.WalkSpeed` (+ (`self.WalkSpeed`) 100.0) :!label _label_6))
      (set `self.SprintSpeed` (+ (`self.SprintSpeed`) 200.0))
      (set `CharacterMovementComponent.MaxWalkSpeed` _output_get_3 (`self.CharacterMovement`)))
    (:`NewEnumerator15`
      (goto _label_6))))

(event `Lvl up`
  (set `self.XP` 0.0)
  (set `self.XP to lvl up` (+ (`self.XP to lvl up`) 15.0))
  (set `self.SkillPoints` (+ (`self.SkillPoints`) 1)))

(event `Save Skill Tree`
  (`KismetArrayLibrary.Array_Clear` (`self.Skills`))
  (for _array_element (`/Game/Blueprints/UserInterface/SkillTree/WB_SkillTree.Skills Array` (`self.SkillTreeWidget`))
    (`KismetArrayLibrary.Array_Append` (`self.Skills`) (`|MakeArray` (`/Game/Blueprints/UserInterface/SkillTree/WB_Skill.SkillUnlocked` _array_element)))))

(event `EnhancedInput|/Game/Inputs/IA_Hotbar1`
  (params (ActionValue :type Boolean) (ElapsedSeconds :type "Float (double-precision)") (TriggeredSeconds :type "Float (double-precision)") (InputAction :type "InputAction Object Reference" :default "/Game/Inputs/IA_Hotbar1.IA_Hotbar1"))
  (:`Triggered`
    (`self.Set Active Hotbar Index` 0)))

(event `EnhancedInput|/Game/Inputs/IA_Hotbar2`
  (params (ActionValue :type Boolean) (ElapsedSeconds :type "Float (double-precision)") (TriggeredSeconds :type "Float (double-precision)") (InputAction :type "InputAction Object Reference" :default "/Game/Inputs/IA_Hotbar2.IA_Hotbar2"))
  (:`Triggered`
    (`self.Set Active Hotbar Index` 1)))

(event `EnhancedInput|/Game/Inputs/IA_ViewAchievements`
  (params (ActionValue :type Boolean) (ElapsedSeconds :type "Float (double-precision)") (TriggeredSeconds :type "Float (double-precision)") (InputAction :type "InputAction Object Reference" :default "/Game/Inputs/IA_ViewAchievements.IA_ViewAchievements"))
  (bind _achievementswidget (`self.AchievementsWidget`))
  (:`Started`
    (bind _achievementswidget_2 (`self.AchievementsWidget`)
      (:`then`
        (`Widget.RemoveFromParent` _achievementswidget_2)
        (set `self.AchievementsWidget` null))
      (:`else`
        (bind _returnvalue (`|CreateWidget` "/Game/Blueprints/UserInterface/Achievements/WB_Achievements.WB_Achievements_C"))
        (bind _output_get (set `self.AchievementsWidget` _returnvalue))
        (`UserWidget.AddToViewport` _output_get 0)
        (set `/Game/Blueprints/UserInterface/Achievements/WB_Achievements.Player` self _achievementswidget)
        (`/Game/Blueprints/UserInterface/Achievements/WB_Achievements.Show Achievements` _achievementswidget)))))

(event `EnhancedInput|/Game/Inputs/IA_Hotbar3`
  (params (ActionValue :type Boolean) (ElapsedSeconds :type "Float (double-precision)") (TriggeredSeconds :type "Float (double-precision)") (InputAction :type "InputAction Object Reference" :default "/Game/Inputs/IA_Hotbar3.IA_Hotbar3"))
  (:`Triggered`
    (`self.Set Active Hotbar Index` 2)))

(event `EnhancedInput|/Game/Inputs/IA_Hotbar4`
  (params (ActionValue :type Boolean) (ElapsedSeconds :type "Float (double-precision)") (TriggeredSeconds :type "Float (double-precision)") (InputAction :type "InputAction Object Reference" :default "/Game/Inputs/IA_Hotbar4.IA_Hotbar4"))
  (:`Triggered`
    (`self.Set Active Hotbar Index` 3)))

(fn `CanAttack`
  (returns (CanAttack :type Boolean))
  (return (> (- (`KismetSystemLibrary.GetGameTimeInSeconds`) (`self.LastAttackedTime`)) (`self.AttackCooldown`))))

(fn `Detect Hits`
  (returns (Hits :type "Array of HitResult Structure"))
  (bind (_returnvalue_location _returnvalue_rotation) (`KismetMathLibrary.BreakTransform` (`SceneComponent.K2_GetComponentToWorld` (`self.Camera`))))
  (bind _outhits (`KismetSystemLibrary.LineTraceMulti` :`Start` _returnvalue_location :`End` (+ _returnvalue_location (* (`KismetMathLibrary.GetForwardVector` _returnvalue_rotation) (`self.HitReach`))) :`TraceChannel` "TraceTypeQuery1" :`DrawDebugType` "ForDuration" :`TraceColor` (struct :`R` 1.0 :`G` 0.987288 :`A` 1.0)))
  (return _outhits))

(fn `DetectAndHitActors`
  (bind _hits (`self.Detect Hits`))
  (for _array_element _hits
    (bind _asbp_base_resource (cast `/Game/Blueprints/Structures/Resources/BP_BaseResource` (`.HitActor` (`GameplayStatics.BreakHitResult` _array_element))))
    (`self.HitResource` _asbp_base_resource)))

(fn `GetActiveTool`
  (returns (Tool :type "/Game/Blueprints/DataStructs/STR_Tool Structure"))
  (bind _bpc_inventorycomponent (`self.BPC_InventoryComponent`))
  (bind _itemstack_itemid (break `/Game/Blueprints/DataStructs/STR_ItemStack` (`/Game/Blueprints/Components/BPC_InventoryComponent.GetHotberItem` _bpc_inventorycomponent (`/Game/Blueprints/Components/BPC_InventoryComponent.ActiveHotbarIndex` _bpc_inventorycomponent))))
  (bind _returnvalue (`|GetDataTableRow` "/Game/Blueprints/DataStructs/DT_Tools.DT_Tools" _itemstack_itemid)
    (:`then`
      (return _returnvalue))
    (:`RowNotFound`
      (return (make `/Game/Blueprints/DataStructs/STR_Tool` "NewEnumerator2")))))

(fn `GetProportions`
  (returns (OutProportions :type "/Game/Blueprints/DataStructs/STR_CharacterProportions Structure"))
  (return (`self.BodyProportions`)))

(fn `HitResource`
  (params (HitResource :type "/Game/Blueprints/Structures/Resources/BP_BaseResource Object Reference"))
  (`/Game/Blueprints/Interfaces/BPI_HarvestableResource.Harvest` HitResource (`self.BPC_InventoryComponent`) (`self.GetActiveTool`)))

(fn `InitializeAttack`
  (if (`self.CanAttack`)
    (`self.PlayAnimMontage` "/Game/Animations/Player/HitAnimationMontage1.HitAnimationMontage1" 5.0)
    (set `self.LastAttackedTime` (`KismetSystemLibrary.GetGameTimeInSeconds`))))

(fn `LineTraceFromSelf`
  (params (LineTraceMaxDistance :type "Float (double-precision)"))
  (returns (OutHit :type "Actor Object Reference"))
  (bind (_returnvalue_location _returnvalue_rotation) (`KismetMathLibrary.BreakTransform` (`SceneComponent.K2_GetComponentToWorld` (`self.Camera`))))
  (bind _outhit (`KismetSystemLibrary.LineTraceSingle` :`Start` _returnvalue_location :`End` (+ _returnvalue_location (* (`KismetMathLibrary.GetForwardVector` _returnvalue_rotation) (`local.LineTraceMaxDistance`))) :`TraceChannel` "TraceTypeQuery1" :`DrawDebugType` "ForOneFrame"))
  (return (`.HitActor` (`GameplayStatics.BreakHitResult` _outhit))))

(fn `PickupItem`
  (bind _focusedpickup (`self.FocusedPickup`))
  (`/Engine/EditorBlueprintResources/StandardMacros.IsValid` _focusedpickup
    (:`Is Valid`
      (`/Game/Blueprints/Components/BPC_InventoryComponent.Add Item Stack` (`self.BPC_InventoryComponent`) (`/Game/Blueprints/Items/BP_WorldItemPickup.ItemStack` _focusedpickup))
      (`self.K2_DestroyActor` (`self.FocusedPickup`))
      (set `self.FocusedPickup` null))))

(fn `Resolve Interact`
  (bind _outhit (`self.LineTraceFromSelf` (`self.InteractReach`)))
  (bind _asbt_chest_bottom_top (cast `/Game/Blueprints/Structures/Chests/BT_ChestBottom_Top` _outhit)
    (:`then`
      (if (`/Game/Blueprints/Structures/Chests/BT_ChestBottom_Top.IsClosed` _asbt_chest_bottom_top)
        (`/Game/Blueprints/Structures/Chests/BT_ChestBottom_Top.OpenChest` _asbt_chest_bottom_top)
        (set `/Game/Blueprints/Structures/Chests/BT_ChestBottom_Top.IsClosed` false _asbt_chest_bottom_top)
        (`KismetSystemLibrary.PrintString` "Openning")))
    (:`CastFailed`
      (`/Engine/EditorBlueprintResources/StandardMacros.IsValid` (`self.FocusedPickup`)
        (:`Is Valid`
          (`self.PickupItem`))
        (:`Is Not Valid`
          (bind _asbpi_interactable (cast `/Game/Blueprints/Interfaces/BPI_Interactable` _outhit))
          (`/Game/Blueprints/Interfaces/BPI_Interactable.Interact` _asbpi_interactable self))))))

(fn `Resolve Oxygen`
  (bind (_returnvalue_x _returnvalue_y _returnvalue_z) (`KismetMathLibrary.BreakVector` (`self.K2_GetActorLocation`)))
  (if (`self.IsInWater`)
    (if (> (`self.OxygenNow`) 0.0)
      (bind _output_get (set `self.OxygenNow` (- (`self.OxygenNow`) 1.0)))
      (`self.OxygenUpdated` (`self.MaxOxygen`) _output_get)
      (else
        (`GameplayStatics.ApplyDamage` self 0.2)))
    (elif (not (>= (`self.OxygenNow`) (`self.MaxOxygen`)))
      (bind _output_get_2 (set `self.OxygenNow` (+ (`self.OxygenNow`) 1.0)))
      (`self.OxygenUpdated` (`self.MaxOxygen`) _output_get_2)))
  (if (< _returnvalue_z -1550.0)
    (if (not (`self.IsInWater`))
      (set `self.IsInWater` true))
    (elif (`self.IsInWater`)
      (set `self.IsInWater` false))))

(fn `ResolveDroppedItemFocusWidget`
  (params (LineTraceHitActor :type "Actor Object Reference"))
  (bind _asbp_world_item_pickup (cast `/Game/Blueprints/Items/BP_WorldItemPickup` LineTraceHitActor)
    (:`then`
      (bind _output_get (set `self.FocusedPickup` _asbp_world_item_pickup))
      (bind (_outicon _outquantity) (`/Game/Blueprints/Items/BP_WorldItemPickup.GetItemDisplayInfo` _output_get))
      (`/Game/Blueprints/UserInterface/WB_ItemFocusInfo.Update` (`self.ItemFocusWidget`) _outquantity _outicon)
      (`/Game/Blueprints/UserInterface/WB_ItemFocusInfo.SetVisible` (`self.ItemFocusWidget`)))
    (:`CastFailed`
      (`/Game/Blueprints/UserInterface/WB_ItemFocusInfo.SetHidden` (`self.ItemFocusWidget`))
      (set `self.FocusedPickup` null))))

(fn `ResolveHoverOnActors`
  (locals (LineTraceHit :type "Actor Object Reference"))
  (bind _output_get (set `local.LineTraceHit` (`self.LineTraceFromSelf` (`self.InteractReach`))))
  (`self.ResolveDroppedItemFocusWidget` _output_get)
  (`self.ResolveInteractTooltip` (`local.LineTraceHit`)))

(fn `ResolveInteractTooltip`
  (params (LineTraceHitActor :type "Actor Object Reference"))
  (bind _interacttooltipwidget (`self.InteractTooltipWidget`))
  (bind _asbpi_interactable (cast `/Game/Blueprints/Interfaces/BPI_Interactable` LineTraceHitActor)
    (:`then`
      (bind _interacthint (`/Game/Blueprints/Interfaces/BPI_Interactable.GetInteractHint` _asbpi_interactable))
      (`/Game/Blueprints/UserInterface/WBP_InteractTooltip.SetText` _interacttooltipwidget _interacthint)
      (`/Game/Blueprints/UserInterface/WBP_InteractTooltip.SetVisible` _interacttooltipwidget))
    (:`CastFailed`
      (`/Game/Blueprints/UserInterface/WBP_InteractTooltip.SetHidden` _interacttooltipwidget))))

(fn `Set Active Hotbar Index`
  (params (index :type Integer))
  (bind _index (`local.index`))
  (bind _bpc_buildsystem (`self.BPC_BuildSystem`))
  (bind _itemstack_itemid (break `/Game/Blueprints/DataStructs/STR_ItemStack` (`/Game/Blueprints/Components/BPC_InventoryComponent.GetHotberItem` (`self.BPC_InventoryComponent`) index)))
  (`/Game/Blueprints/BPC_BuildSystem.Stop Build Mode` (`self.BPC_BuildSystem`))
  (`KismetSystemLibrary.PrintString` "Sett")
  (bind _returnvalue (`|GetDataTableRow` "/Game/Blueprints/DataStructs/DT_Items.DT_Items" _itemstack_itemid)
    (:`then`
      (`StaticMeshComponent.SetStaticMesh` (`self.ToolMesh`) (`.WroldMesh_22_CEB77EF144632406D06AF783E98E4173` (break `/Game/Blueprints/DataStructs/STR_ItemData` _returnvalue)))
      (`SceneComponent.SetWorldScale3D` (`self.ToolMesh`) (`KismetMathLibrary.Conv_DoubleToVector` (`.WorldMeshScale_25_67BC7ABD45144958CBF588B18A2E6809` (break `/Game/Blueprints/DataStructs/STR_ItemData` _returnvalue)))))
    (:`RowNotFound`
      (`StaticMeshComponent.SetStaticMesh` (`self.ToolMesh`) null)))
  (set `/Game/Blueprints/Components/BPC_InventoryComponent.ActiveHotbarIndex` _index (`self.BPC_InventoryComponent`))
  (`KismetSystemLibrary.PrintString` (`KismetStringLibrary.Conv_IntToString` _index))
  (bind _returnvalue_2 (`|GetDataTableRow` "/Game/Blueprints/DT_BuildParts.DT_BuildParts" (break `/Game/Blueprints/DataStructs/STR_ItemData` _returnvalue))
    (:`then`
      (set `/Game/Blueprints/BPC_BuildSystem.buildable index` (`KismetArrayLibrary.Array_Find` (`/Game/Blueprints/BPC_BuildSystem.DT_Buildables` _bpc_buildsystem) _returnvalue_2) _bpc_buildsystem)
      (`/Game/Blueprints/BPC_BuildSystem.EnterBuildMode` _bpc_buildsystem))))

(fn `Sprint`
  (set `CharacterMovementComponent.MaxWalkSpeed` (`self.SprintSpeed`) (`self.CharacterMovement`)))

(fn `StopSprint`
  (set `CharacterMovementComponent.MaxWalkSpeed` (`self.WalkSpeed`) (`self.CharacterMovement`)))

(fn `UserConstructionScript`)