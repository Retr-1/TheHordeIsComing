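; Master power-up pickup that permanently raises a player character's stats on overlap, then destroys itself.
; A timeline started on BeginPlay animates the mesh's relative height.
; Overlap with a "Player"-tagged BP_BaseCharacter calls AddPowerUp, which scales jump velocity, max health, walk speed and sprint speed up by multiplier variables.
; Each increase is a fraction of the current value, so repeated pickups compound.
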(event `self.ReceiveBeginPlay`
  (bind (_direction _opencurve) (`Timeline|Timeline`)
    (:`Update`
      (`SceneComponent.K2_SetRelativeLocation` (`self.StaticMesh`) (`KismetMathLibrary.MakeVector` 0.0 0.0 (* _opencurve 100.0)) false false))))

(event `self.ReceiveActorBeginOverlap`
  (params (OtherActor :type "Actor Object Reference"))
  (if (`self.ActorHasTag` OtherActor "Player")
    (bind _asbp_base_character (cast `/Game/Blueprints/BP_BaseCharacter` OtherActor))
    (set `self.Other Actor` _asbp_base_character)
    (`self.AddPowerUp`)
    (`self.K2_DestroyActor`)))

(fn `AddPowerUp`
  (bind _other_actor (`self.Other Actor`))
  (bind _other_actor_2 (`self.Other Actor`))
  (bind _speedmult (`self.SpeedMult`))
  (bind _maxhealth (`/Game/Blueprints/BP_BaseCharacter.MaxHealth` _other_actor))
  (bind _walkspeed (`/Game/Blueprints/BP_BaseCharacter.WalkSpeed` _other_actor_2))
  (bind _sprintspeed (`/Game/Blueprints/BP_BaseCharacter.SprintSpeed` _other_actor_2))
  (bind _charactermovement (`Character.CharacterMovement` (`self.Other Actor`)))
  (bind _jumpzvelocity (`CharacterMovementComponent.JumpZVelocity` _charactermovement))
  (set `CharacterMovementComponent.JumpZVelocity` (+ _jumpzvelocity (* _jumpzvelocity (`self.JumpMult`))) _charactermovement)
  (set `/Game/Blueprints/BP_BaseCharacter.MaxHealth` (+ _maxhealth (* _maxhealth (`self.MaxHealthMult`))) _other_actor)
  (set `/Game/Blueprints/BP_BaseCharacter.WalkSpeed` (+ (* _walkspeed _speedmult) _walkspeed) _other_actor_2)
  (set `/Game/Blueprints/BP_BaseCharacter.SprintSpeed` (+ (* _sprintspeed _speedmult) _sprintspeed) _other_actor_2))

(fn `UserConstructionScript`)